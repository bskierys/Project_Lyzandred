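; BP_Key is a key pickup actor with a configurable mesh and a switchable glow.
; The construction script applies KeyMesh to KeyVisuals, while BeginPlay and the Start/StopGlowing events pass the IsGlowing state to that component.
; On any actor overlap it broadcasts the KeyDefinition's KeyId on the key-collected event channel, then calls CollectKey with the overlapping actor.
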(event Custom|StartGlowing
  (bind _output_get (Variables|Key|SetbIsGlowing true))
  (Variables|/Game/Lyzandred/Blueprints/Props/BP_GlowingStatickMesh.BP_GlowingStatickMesh_C|SetbIsGlowActive (Variables|Default|GetKeyVisuals) _output_get))

(event Custom|StopGlowing
  (bind _output_get (Variables|Key|SetbIsGlowing false))
  (Variables|/Game/Lyzandred/Blueprints/Props/BP_GlowingStatickMesh.BP_GlowingStatickMesh_C|SetbIsGlowActive (Variables|Default|GetKeyVisuals) _output_get))

(event EventBeginPlay
  (Variables|/Game/Lyzandred/Blueprints/Props/BP_GlowingStatickMesh.BP_GlowingStatickMesh_C|SetbIsGlowActive (Variables|Default|GetKeyVisuals) (Variables|Key|GetbIsGlowing)))

(event Collision|EventActorBeginOverlap
  (params (OtherActor :type Actor%20Object%20Reference))
  (Class|EventSubsystem|SendEvent (Subsystems|GetEventSubsystem) "/Game/Lyzandred/Blueprints/Events/DA_KeyCollectedChannel.DA_KeyCollectedChannel" (Variables|/Script/Project_Lyzandred.Lyz_KeyDefinition|GetKeyId (Variables|Default|GetKeyDefinition)) self)
  (Class|LyzKey|CollectKey OtherActor))

(fn ConstructionScript
  (Components|StaticMesh|SetStaticMesh (Variables|Default|GetKeyVisuals) (Variables|Default|GetKeyMesh)))