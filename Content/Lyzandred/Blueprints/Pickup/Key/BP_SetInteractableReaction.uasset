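; BP_SetInteractableReaction is a key-related reaction that switches an actor's interactability on or off.
; ExecuteReaction finds the first BP_InteractableComponent on the given actor and passes ShouldUnlock to its SetEnabled.
; Actors without that component are left untouched through a validity check.
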(event EventExecuteReaction
  (params (Actor :type Actor%20Object%20Reference) (bShouldUnlock :type Boolean))
  (bind _interactablecomponent (CallFunction|ExtractInteractableComponent Actor))
  (Utilities|IsValid _interactablecomponent
    (:Is%20Valid
      (Default|SetEnabled _interactablecomponent bShouldUnlock))))

(fn ExtractInteractableComponent
  (params (Actor :type Actor%20Object%20Reference))
  (bind _returnvalue (Actor|GetComponentsByClass Actor "/Game/Lyzandred/Blueprints/Props/Interactable/BP_InteractableComponent.BP_InteractableComponent_C"))
  (if (> (Utilities|Array|Length _returnvalue) 0)
    (return (Utilities|Array|Get(acopy) _returnvalue))
    (else
      (return 0))))