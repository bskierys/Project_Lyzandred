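; Component that locks or unlocks its owning actor based on a list of required keys stored in the game state.
; After a one-tick delay on BeginPlay, it runs its UnlockReaction with the current result and subscribes to key changes.
; Changes to a required key re-run the reaction, which unlocks only when all keys are set.
; A helper combines every key's LockedReason into one message, including those already met.
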(event Custom|OnFlagChanged
  (params (Key :type Name) (Value :type Boolean))
  (bind _unlockreaction (Variables|Default|GetUnlockReaction))
  (if (CallFunction|DoesRequiredKeysContainId Key)
    (Utilities|IsValid _unlockreaction
      (:Is%20Valid
        (Class|LyzUnlockReaction|ExecuteReaction _unlockreaction (Components|GetOwner) (CallFunction|AreRequirementsMet))))))

(event EventBeginPlay
  (bind _unlockreaction (Variables|Default|GetUnlockReaction))
  (|CallParentFunction)
  (Utilities|FlowControl|Delay 0.0)
  (Variables|Default|SetGameStateRef (Class|LyzGameStateLibrary|GetLyzGameState))
  (Utilities|IsValid _unlockreaction
    (:Is%20Valid
      (Class|LyzUnlockReaction|ExecuteReaction _unlockreaction (Components|GetOwner) (CallFunction|AreRequirementsMet))
      (EventDispatchers|BindEventtoOnKeyChanged (Variables|Default|GetGameStateRef) (EventDispatchers|CreateEvent :!event Custom|OnFlagChanged)))))

(event EventEndPlay
  (params (EndPlayReason :type EEndPlayReason%20Enum :default "Destroyed"))
  (EventDispatchers|UnbindEventfromOnKeyChanged (Variables|Default|GetGameStateRef) (delegate Custom|OnFlagChanged)))

(fn AreRequirementsMet
  (for _array_element (Variables|Default|GetRequiredKeys)
    (if (not (Class|LyzGameState|GetKey (Variables|Default|GetGameStateRef) (Variables|/Script/Project_Lyzandred.Lyz_KeyDefinition|GetKeyId _array_element)))
      (return false)))
  (return true))

(fn DoesRequiredKeysContainId
  (params (FlagId :type Name))
  (for _array_element (Variables|Default|GetRequiredKeys)
    (if (== FlagId (Variables|/Script/Project_Lyzandred.Lyz_KeyDefinition|GetKeyId _array_element))
      (return true)))
  (return false))

(fn CreateWhyLockedMessage
  (for _array_element (Variables|Default|GetRequiredKeys)
    (Utilities|Array|Add (LocalVariables|GetTextsArray) (Variables|/Script/Project_Lyzandred.Lyz_KeyDefinition|GetLockedReason _array_element)))
  (bind _message (CallFunction|ArrayOfTextstoText (LocalVariables|GetTextsArray)))
  (return _message))