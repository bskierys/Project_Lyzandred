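; Base coin pickup that, when overlapped by the current player pawn while interactable, reports its CoinType to the game mode, plays a sound and destroys itself.
; AnimateCoinSpawn waits a given delay, reveals the mesh and runs a pop timeline that scales the sphere and offsets its height from the location cached at BeginPlay.
; Pickup is enabled when the pop finishes, while Show and Hide toggle visibility and interactability directly.
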(event EventBeginPlay
  (Variables|Default|SetPlacedLocation (Transformation|GetWorldLocation (Variables|Default|GetSphere))))

(event EventAnimateCoinSpawn
  (params (Delay :type Float%20%28single-precision%29))
  (Utilities|FlowControl|Delay Delay)
  (Rendering|SetVisibility (Variables|Default|GetStaticMesh) true false)
  ;[0.15 0.15 0.15 0.5] Coin Pop Animation
  (bind (_direction _scale _offsetz) (Timeline|Spawn%20Anim%20Timeline Play)
    (:Update
      (Utilities|IsValid (Variables|Default|GetSphere)
        (:Is%20Valid
          (Transformation|SetWorldScale3D (Variables|Default|GetSphere) (Math|Vector|MakeVector _scale _scale _scale))
          (Utilities|IsValid (Variables|Default|GetSphere)
            (:Is%20Valid
              (Transformation|SetWorldLocation (Variables|Default|GetSphere) (CallFunction|ComputeAnimCoinNewLocation _offsetz) false false))))))
    (:Finished
      ;[0.15 0.15 0.15 0.5] Set Interactable so that we can pick it up
      (Variables|Default|SetbIsInteractable true))))

(event EventShow
  ;[0.15 0.15 0.15 0.5] Visibility
  (Variables|Default|SetbIsInteractable true)
  (Rendering|SetVisibility (Variables|Default|GetStaticMesh) true false))

(event EventHide
  ;[0.15 0.15 0.15 0.5] Visibility
  (Variables|Default|SetbIsInteractable false)
  (Rendering|SetVisibility (Variables|Default|GetStaticMesh) false false))

(event Collision|EventActorBeginOverlap
  (params (OtherActor :type Actor%20Object%20Reference))
  ;[0.15 0.15 0.15 0.5] Check if overlaps with the character
  (if (and (Class|LyzCharacterHelperLibrary|CheckifCurrentPlayerPawn OtherActor) (Variables|Default|GetbIsInteractable))
    (Class|BPIPickupManager|AddCoin(Message) (Game|GetGameMode) (Variables|Default|GetCoinType))
    (Audio|PlaySoundatLocation "/Game/Lyzandred/Assets/SFX/SFX_CoinPickup_Cue.SFX_CoinPickup_Cue" (Transformation|GetActorLocation) "0, 0, 0" 1.0 1.0 0.0 0 0 0 0)
    (Actor|DestroyActor)))

(fn ConstructionScript)

(fn ComputeAnimCoinNewLocation
  (params (OffsetZ :type Float%20%28double-precision%29))
  (bind _placedlocation (Variables|Default|GetPlacedLocation))
  (bind (_x _y _z) (Math|Vector|BreakVector _placedlocation))
  (return (Math|Vector|MakeVector _x _y (+ _z OffsetZ))))