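; BP_SwitchOnOnLoadComponent is an actor component that switches its owner on and off as a level loads and unloads.
; On BeginPlay it binds to the loaded and unloaded events of a LevelLoader, if one is valid, and unbinds them on EndPlay.
; Each event relays to the owner as a SwitchOnMessage or SwitchOffMessage call, linking level streaming state to the owner's switch behaviour.
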(event Custom|OnLevelLoaded
  (params (Loader :type Lyz%20Level%20Loader%20Object%20Reference))
  (Class|LyzSwitchableInterface|Switchon(Message) (Components|GetOwner)))

(event Custom|OnLevelUnloaded
  (params (Loader :type Lyz%20Level%20Loader%20Object%20Reference))
  (Class|LyzSwitchableInterface|SwitchOff(Message) (Components|GetOwner)))

(event EventBeginPlay
  (if (Utilities|IsValid (Variables|Default|GetLevelLoader))
    (EventDispatchers|BindEventtoOnLevelLoaded (Variables|Default|GetLevelLoader) (EventDispatchers|CreateEvent :!event Custom|OnLevelLoaded))
    (EventDispatchers|BindEventtoOnLevelUnLoaded (Variables|Default|GetLevelLoader) (EventDispatchers|CreateEvent :!event Custom|OnLevelUnloaded))))

(event EventEndPlay
  (params (EndPlayReason :type EEndPlayReason%20Enum :default "Destroyed"))
  (EventDispatchers|UnbindEventfromOnLevelLoaded (Variables|Default|GetLevelLoader) (delegate Custom|OnLevelLoaded))
  (EventDispatchers|UnbindEventfromOnLevelUnLoaded (Variables|Default|GetLevelLoader) (delegate Custom|OnLevelUnloaded)))