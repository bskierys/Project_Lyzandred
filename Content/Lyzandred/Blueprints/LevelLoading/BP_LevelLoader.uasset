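; BP_LevelLoader is a trigger actor that streams a level in or out as the current player pawn crosses it.
; On the pawn's begin and end overlap it records the pawn's offset along the actor's forward vector using a dot product, with a DoOnce guarding the entry value.
; A forward crossing loads the level asynchronously and makes it visible, a backward one unloads it, and each operation sends a notification.
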(event EventLoadLevel
  (Class|GameplayStatics|LoadStreamLevelbySoftObjectPtr (Variables|Default|GetLevelToLoad) true false)
  (Class|LyzLevelLoader|NotifyLevelLoaded))

(event Collision|EventActorBeginOverlap
  (params (OtherActor :type Actor%20Object%20Reference))
  ;[0.15 0.15 0.15 0.5] Load/Unload when character crosses
  (if (Class|LyzCharacterHelperLibrary|CheckifCurrentPlayerPawn OtherActor)
    (Utilities|FlowControl|DoOnce false
      (:Completed
        (Variables|Default|SetEntryDot (CallFunction|GetCurrentDotOffset))))))

(event Collision|EventActorEndOverlap
  (params (OtherActor :type Actor%20Object%20Reference))
  ;[0.15 0.15 0.15 0.5] Load/Unload when character crosses
  (if (Class|LyzCharacterHelperLibrary|CheckifCurrentPlayerPawn OtherActor)
    (Utilities|FlowControl|Sequence
      (:then_0
        (Utilities|FlowControl|DoOnce false) ; enters at Reset
      )
      (:then_1
        (bind _output_get (Variables|Default|SetExitDot (CallFunction|GetCurrentDotOffset)))
        (switch Utilities|FlowControl|Switch|SwitchonETraversalDirection (Class|LyzLevelLoader|ComputeCrossDirection (Variables|Default|GetEntryDot) _output_get)
          (:Forward
            (Class|LyzLevelLoader|LoadLevel))
          (:Backward
            (Class|LyzLevelLoader|UnLoadLevel)))))))

(event EventUnLoadLevel
  (Class|GameplayStatics|UnloadStreamLevelbySoftObjectPtr (Variables|Default|GetLevelToLoad) false)
  (Class|LyzLevelLoader|NotifyLevelUnLoaded))

(fn ConstructionScript)

(fn GetCurrentDotOffset
  (return (Math|Vector|DotProduct (- (Transformation|GetActorLocation (Game|Player|GetPlayerPawn 0)) (Transformation|GetActorLocation self)) (Transformation|GetActorForwardVector))))