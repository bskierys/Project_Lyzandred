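; BP_LevelLoadingManager keeps one level active by coordinating the level loaders placed in the level.
; The C++ parent fills the loader list, and BeginPlay waits on a zero-second Delay as a workaround so that runs before binding to each loader's OnLevelLoaded.
; When a loader reports its level loaded, the manager stores it as ActiveLoader and tells every other loader to unload.
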(event Custom|OnLevelLoaded
  (params (Loader :type Lyz%20Level%20Loader%20Object%20Reference))
  ;[0.15 0.15 0.15 0.5] When Level is Loaded, unload all the others and broadcast to reactors
  (Variables|Default|SetActiveLoader Loader)
  (for _array_element (Variables|Default|GetLevelLoadersOnLevel)
    (if (not (== _array_element (Variables|Default|GetActiveLoader)))
      (Class|LyzLevelLoader|UnLoadLevel _array_element))))

(event EventBeginPlay
  ;[0.15 0.15 0.15 0.5] Loaders on Level are populated in C++
  (|CallParentFunction)
  ;[0.15 0.15 0.15 0.5] Workaround to make C++ parent be called before the loop.
  (Utilities|FlowControl|Delay 0.0)
  ;[0.15 0.15 0.15 0.5] Assign Events to react
  (for _array_element (Variables|Default|GetLevelLoadersOnLevel)
    (EventDispatchers|BindEventtoOnLevelLoaded _array_element (EventDispatchers|CreateEvent :!event Custom|OnLevelLoaded))))

(fn ConstructionScript)