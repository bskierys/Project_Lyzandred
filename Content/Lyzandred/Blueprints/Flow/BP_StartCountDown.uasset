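; BP_StartCountDown is a trigger actor that starts a countdown when the player pawn overlaps it.
; It passes CountdownTime and a finish callback to the timer subsystem, then shows the timer message on the HUD.
; When time runs out, it prints a message, plays a whistle, waits briefly, and hides the HUD timer unless a countdown is running again.
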(event Custom|OnTimerFinished
  (Development|PrintString "Time's up!")
  (Audio|PlaySound2D "/Game/Lyzandred/Assets/SFX/SFX_AttentionWhistle.SFX_AttentionWhistle" 1.0 1.0 0.0 0 0)
  (Utilities|FlowControl|Delay 3.0)
  (if (not (Class|TimerSubsystem|IsRunning (Subsystems|GetTimerSubsystem)))
    (Class|BPIHud|SetTimerVisibility(Message) (HUD|GetHUD (Game|GetPlayerController 0)) "Hidden")))

(event Collision|EventActorBeginOverlap
  (params (OtherActor :type Actor%20Object%20Reference))
  (if (== OtherActor (Game|Player|GetPlayerPawn 0))
    (Class|TimerSubsystem|StartCountdown (Subsystems|GetTimerSubsystem) (Variables|Default|GetCountdownTime) (EventDispatchers|CreateEvent :!event Custom|OnTimerFinished))
    (Class|BPIHud|SetTimerVisibility(Message) (HUD|GetHUD (Game|GetPlayerController 0)) "Visible")))

(fn ConstructionScript)