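; BP_StopTimer is a trigger actor that stops the game timer when the player pawn overlaps it.
; It calls StopTimer on the timer subsystem, then waits a few seconds.
; If the timer is still not running after the delay, it tells the player's HUD to hide the timer, so a timer restarted in the meantime is left alone.
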(event Collision|EventActorBeginOverlap
  (params (OtherActor :type Actor%20Object%20Reference))
  (if (== OtherActor (Game|Player|GetPlayerPawn 0))
    (Class|TimerSubsystem|StopTimer (Subsystems|GetTimerSubsystem))
    (Utilities|FlowControl|Delay 3.0)
    (if (not (Class|TimerSubsystem|IsRunning (Subsystems|GetTimerSubsystem)))
      (Class|BPIHud|SetTimerVisibility(Message) (HUD|GetHUD (Game|GetPlayerController 0)) "Hidden"))))

(fn ConstructionScript)