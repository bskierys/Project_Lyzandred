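; Patrol target actor for enemies that defines a circular area by Radius and senses actors inside it.
; Overlap events maintain the ActorsInArea set and broadcast OnActorSensedInArea on entry and exit, while FindActorInArea filters that set by class.
; The construction script sizes the EnterDetection sphere to Radius.
; GetRandomPointOnGround picks a random angle and distance at the actor's height without tracing, so points cluster toward the centre.
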(event EventBeginPlay)

(event Collision|EventActorBeginOverlap
  (params (OtherActor :type Actor%20Object%20Reference))
  (Utilities|Set|Add (Variables|Default|GetActorsInArea) OtherActor)
  (Default|CallOnActorSensedinArea OtherActor true))

(event Collision|EventActorEndOverlap
  (params (OtherActor :type Actor%20Object%20Reference))
  (Utilities|Set|Remove (Variables|Default|GetActorsInArea) OtherActor)
  (Default|CallOnActorSensedinArea OtherActor false))

(event EventEndPlay
  (params (EndPlayReason :type EEndPlayReason%20Enum :default "Destroyed"))
  (EventDispatchers|UnbindallEventsfromOnActorSensedinArea))

(fn ConstructionScript
  ;[0.15 0.15 0.15 0.5] For Debug Purposes
  (Components|Sphere|SetSphereRadius (Variables|Default|GetEnterDetection) (Variables|Default|GetRadius) true)
  (Rendering|SetActorHiddenInGame false))

(fn GetRandomPointonGround
  (LocalVariables|SetAngle (Math|Random|RandomFloatinRange 0.0 (Math|Float|MultiplybyPi 2.0)))
  (LocalVariables|SetDistance (Math|Random|RandomFloatinRange 0.0 (Variables|Default|GetRadius)))
  (return (+ (Math|Vector|MakeVector (* (Math|Trig|Cos(Radians) (LocalVariables|GetAngle)) (LocalVariables|GetDistance)) (* (Math|Trig|Sin(Radians) (LocalVariables|GetAngle)) (LocalVariables|GetDistance)) 0.0) (Transformation|GetActorLocation))))

(fn FindActorinArea
  (params (ActorClass :type Actor%20Class%20Reference))
  (bind _found (LocalVariables|GetFound))
  (bind _result (Utilities|Set|ToArray (Variables|Default|GetActorsInArea)))
  (for _array_element _result
    (if (Class|GameplayStatics|ObjectIsA _array_element ActorClass)
      (Utilities|Array|Add (LocalVariables|GetFound) _array_element)))
  (return _found (> (Utilities|Array|Length _found) 0)))