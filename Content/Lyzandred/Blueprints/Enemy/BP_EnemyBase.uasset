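; Base enemy character that melee-attacks, switches alert state, dies on any damage and, given a spawn area, stays hidden until it rises from underground.
; Montage notifies drive the melee component's hit window and spawn reveal, while montage endings broadcast completion events.
; Death notifies the AI controller, disables collision and sends a kill payload through the event subsystem.
; Getters expose the spawn area and passive-behaviour patrol route or wandering point.
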(event Custom|OnAttackHit
  (params (DamagedActor :type Actor%20Object%20Reference))
  ;[0.15 0.15 0.15 0.5] Attack
  (Audio|PlaySoundatLocation "/Game/Lyzandred/Assets/SFX/SFX_SwordHit.SFX_SwordHit" (Transformation|GetActorLocation DamagedActor) "0, 0, 0" 1.0 1.0 0.0 0 0 0 0))

(event EventPlaySpawnAnimation
  ;[0.15 0.15 0.15 0.5] Spawn From Underground
  (if (not (Variables|Default|GetbIsSpawned))
    (Utilities|FlowControl|Delay (Math|Random|RandomFloatinRange 0.0 0.5))
    (bind _notifyname (Animation|Montage|PlayMontage (Variables|Character|GetMesh) "/Game/Lyzandred/Assets/Animations/Enemies/Common/AM_Spawn.AM_Spawn")
      (:OnCompleted
        (Variables|Default|SetbIsSpawned true)
        (Class|LyzEnemy|BroadcastAnimationEnd "Spawn"))
      (:OnNotifyBegin
        (if (== _notifyname "AnimStart")
          (Rendering|SetVisibility (Variables|Character|GetMesh) true true))))))

(event EventPossessed
  (params (NewController :type Controller%20Object%20Reference))
  (bind _asaic_enemy_base (Utilities|Casting|CastToAIC_EnemyBase NewController))
  (Variables|Default|SetEnemyControllerReference _asaic_enemy_base))

(event EventKill
  ;[0.15 0.15 0.15 0.5] Death
  (if (not (Variables|Default|GetbIsDead))
    (Utilities|FlowControl|Sequence
      (:then_0
        (Variables|/Game/Lyzandred/Blueprints/Characters/BP_MeleeAttackComponent.BP_MeleeAttackComponent_C|SetbIsAttackActive (Variables|Default|GetBP_MeleeAttackComponent) false)
        (Audio|PlaySoundatLocation "/Game/Lyzandred/Assets/SFX/SFX_BoneHit.SFX_BoneHit" (Transformation|GetActorLocation) "0, 0, 0" 1.0 1.0 0.2 0 0 0 0)
        (Animation|Montage|PlayMontage (Variables|Character|GetMesh) "/Game/Lyzandred/Assets/Animations/Enemies/Common/AM_DeathSkeletons.AM_DeathSkeletons"
          (:then
            (Default|SetStatetoDead (Variables|Default|GetEnemyControllerReference))
            (Variables|Default|SetbIsDead true)
            (Rendering|Material|SetMaterial (Variables|Character|GetMesh) 1 "/Game/Lyzandred/Assets/Materials/Enemies/MI_GlowingEyesDead.MI_GlowingEyesDead")
            ;;[0.15 0.15 0.15 0.5] Disable collisions for actor to avoid blocking the way
            (Collision|SetCollisionProfileName (Variables|Default|GetCapsuleComponent) "NoCollision" false :!class /Script/Engine.PrimitiveComponent)
            (Collision|SetCollisionProfileName (Variables|Character|GetMesh) "NoCollision" false :!class /Script/Engine.PrimitiveComponent))
          (:OnCompleted
            (AI|Logic|StopLogic (Variables|/Script/AIModule.AIController|GetBrainComponent (Variables|Default|GetEnemyControllerReference)) ""))))
      (:then_1
        ;;[0.15 0.15 0.15 0.5] Propagate the event to the system
        (if (Utilities|IsValidClass (Variables|Default|GetEnemyType))
          (bind _returnvalue (Game|ConstructObjectfromClass "/Game/Lyzandred/Blueprints/Events/BP_KillEnemyPayload.BP_KillEnemyPayload_C"))
          (Variables|/Game/Lyzandred/Blueprints/Events/BP_KillEnemyPayload.BP_KillEnemyPayload_C|SetEnemyTags _returnvalue (Variables|Default|GetTags))
          (Variables|/Game/Lyzandred/Blueprints/Events/BP_KillEnemyPayload.BP_KillEnemyPayload_C|SetEnemyType _returnvalue (Variables|Default|GetEnemyType))
          (Class|EventSubsystem|SendEvent (Subsystems|GetEventSubsystem) "/Game/Lyzandred/Blueprints/Events/DA_KillEnemiesEventChannel.DA_KillEnemiesEventChannel" "KillEnemy" self _returnvalue))))))

(event EventAttack
  ;[0.15 0.15 0.15 0.5] Attack
  (bind _notifyname (Animation|Montage|PlayMontage (Variables|Character|GetMesh) (Variables|Animations|GetAttackMontage))
    (:OnCompleted
      (Class|LyzEnemy|BroadcastAttackEnd :!label _label)
      (Default|AttackWindowClose (Variables|Default|GetBP_MeleeAttackComponent) :!label _label_2))
    (:OnInterrupted
      (goto _label))
    (:OnNotifyBegin
      (switch name _notifyname
        (:AttackStart
          (Default|AttackWindowOpen (Variables|Default|GetBP_MeleeAttackComponent) (Variables|Default|GetBladeDamageArea)))
        (:AttackEnd
          (goto _label_2))))))

(event EventBeginPlay
  (|CallParentFunction)
  (Utilities|FlowControl|Delay 0.0)
  (EventDispatchers|BindEventtoOnAttackHit (Variables|Default|GetBP_MeleeAttackComponent) (EventDispatchers|CreateEvent :!event Custom|OnAttackHit))
  (Utilities|IsValid (Variables|Default|GetSpawnArea)
    (:Is%20Valid
      (Variables|Default|SetbIsSpawned false)
      (Rendering|SetVisibility (Variables|Character|GetMesh) false true))
    (:Is%20Not%20Valid
      (Variables|Default|SetbIsSpawned true))))

(event EventChangeAlertedState
  (params (bNoticeActive :type Boolean) (bWithAnimation :type Boolean))
  ;[0.15 0.15 0.15 0.5] Alerted to Passive
  (if bNoticeActive
    (if bWithAnimation
      (Animation|Montage|PlayMontage (Variables|Character|GetMesh) (Variables|Animations|GetNoticeMontage)
        (:OnCompleted
          _)
        (:OnInterrupted
          _)))
    (Class|LyzEnemy|BroadcastAnimationEnd "Noticed")
    (Variables|Default|SetbIsAlerted true)
    (else
      (if bWithAnimation
        (Animation|Montage|PlayMontage (Variables|Character|GetMesh) (Variables|Animations|GetLostNoticeMontage)
          (:OnCompleted
            _)
          (:OnInterrupted
            _)))
      (Class|LyzEnemy|BroadcastAnimationEnd "LostPlayer")
      (Variables|Default|SetbIsAlerted false))))

(event EventDamage
  ;[0.15 0.15 0.15 0.5] Death
  (if (not (Variables|Default|GetbIsDead))
    (Utilities|FlowControl|Sequence
      (:then_0
        (Variables|/Game/Lyzandred/Blueprints/Characters/BP_MeleeAttackComponent.BP_MeleeAttackComponent_C|SetbIsAttackActive (Variables|Default|GetBP_MeleeAttackComponent) false)
        (Audio|PlaySoundatLocation "/Game/Lyzandred/Assets/SFX/SFX_BoneHit.SFX_BoneHit" (Transformation|GetActorLocation) "0, 0, 0" 1.0 1.0 0.2 0 0 0 0)
        (Animation|Montage|PlayMontage (Variables|Character|GetMesh) "/Game/Lyzandred/Assets/Animations/Enemies/Common/AM_DeathSkeletons.AM_DeathSkeletons"
          (:then
            (Default|SetStatetoDead (Variables|Default|GetEnemyControllerReference))
            (Variables|Default|SetbIsDead true)
            (Rendering|Material|SetMaterial (Variables|Character|GetMesh) 1 "/Game/Lyzandred/Assets/Materials/Enemies/MI_GlowingEyesDead.MI_GlowingEyesDead")
            ;;[0.15 0.15 0.15 0.5] Disable collisions for actor to avoid blocking the way
            (Collision|SetCollisionProfileName (Variables|Default|GetCapsuleComponent) "NoCollision" false :!class /Script/Engine.PrimitiveComponent)
            (Collision|SetCollisionProfileName (Variables|Character|GetMesh) "NoCollision" false :!class /Script/Engine.PrimitiveComponent))
          (:OnCompleted
            (AI|Logic|StopLogic (Variables|/Script/AIModule.AIController|GetBrainComponent (Variables|Default|GetEnemyControllerReference)) ""))))
      (:then_1
        ;;[0.15 0.15 0.15 0.5] Propagate the event to the system
        (if (Utilities|IsValidClass (Variables|Default|GetEnemyType))
          (bind _returnvalue (Game|ConstructObjectfromClass "/Game/Lyzandred/Blueprints/Events/BP_KillEnemyPayload.BP_KillEnemyPayload_C"))
          (Variables|/Game/Lyzandred/Blueprints/Events/BP_KillEnemyPayload.BP_KillEnemyPayload_C|SetEnemyTags _returnvalue (Variables|Default|GetTags))
          (Variables|/Game/Lyzandred/Blueprints/Events/BP_KillEnemyPayload.BP_KillEnemyPayload_C|SetEnemyType _returnvalue (Variables|Default|GetEnemyType))
          (Class|EventSubsystem|SendEvent (Subsystems|GetEventSubsystem) "/Game/Lyzandred/Blueprints/Events/DA_KillEnemiesEventChannel.DA_KillEnemiesEventChannel" "KillEnemy" self _returnvalue))))))

(fn ConstructionScript)

(fn GetPatrolRoute
  (bind _passivebehaviour (Variables|Default|GetPassiveBehaviour))
  (if (and (Class|GameplayStatics|ObjectIsA _passivebehaviour "/Game/Lyzandred/Blueprints/Enemy/Patrol/BP_PatrollingPassiveBehaviour.BP_PatrollingPassiveBehaviour_C") (Utilities|IsValid _passivebehaviour))
    (return (Variables|/Game/Lyzandred/Blueprints/Enemy/Patrol/BP_PatrollingPassiveBehaviour.BP_PatrollingPassiveBehaviour_C|GetPatrolRoute (.AsBP%20Patrolling%20Passive%20Behaviour (Utilities|Casting|CastToBP_PatrollingPassiveBehaviour (Variables|Default|GetPassiveBehaviour)))))))

(fn GetSpawnArea
  (return (Variables|Default|GetSpawnArea)))

(fn GetWanderingPoint
  (bind _passivebehaviour (Variables|Default|GetPassiveBehaviour))
  (if (and (Class|GameplayStatics|ObjectIsA _passivebehaviour "/Game/Lyzandred/Blueprints/Enemy/Patrol/BP_WanderingPassiveBehaviour.BP_WanderingPassiveBehaviour_C") (Utilities|IsValid _passivebehaviour))
    (return (Variables|/Game/Lyzandred/Blueprints/Enemy/Patrol/BP_WanderingPassiveBehaviour.BP_WanderingPassiveBehaviour_C|GetWanderingPoint (.AsBP%20Wandering%20Passive%20Behaviour (Utilities|Casting|CastToBP_WanderingPassiveBehaviour (Variables|Default|GetPassiveBehaviour)))))))