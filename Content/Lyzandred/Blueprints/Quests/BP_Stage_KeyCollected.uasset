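; Quest stage Blueprint that completes when a specific key is collected.
; While listening for completion, it binds to the key-collected channel of the event subsystem, looked up through a data asset.
; Each event's tag is compared to the KeyId of the stage's key definition, and a match completes the stage.
; Clearing the stage runs the parent cleanup and unbinds from the channel.
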(event Custom|OnEvent
  (params (EventTag :type Name) (Sender :type Object%20Object%20Reference) (Payload :type Event%20Payload%20Object%20Object%20Reference))
  (bind _keydefinition (Variables|QuestSubsystem|GetKeyDefinition))
  (Utilities|IsValid _keydefinition
    (:Is%20Valid
      (if (== (Variables|/Script/Project_Lyzandred.Lyz_KeyDefinition|GetKeyId _keydefinition) EventTag)
        (Class|QuestStage|CompleteStage)))))

(event EventListenforCompletion
  (bind _eventsubsystem (Variables|Default|GetEventSubsystem))
  (Utilities|IsValid _eventsubsystem
    (:Is%20Valid
      (EventDispatchers|BindEventtoOnEvent (Class|EventSubsystem|GetEventChannel _eventsubsystem "/Game/Lyzandred/Blueprints/Events/DA_KeyCollectedChannel.DA_KeyCollectedChannel") (EventDispatchers|CreateEvent :!event Custom|OnEvent)))))

(event EventClear
  (bind _eventsubsystem (Variables|Default|GetEventSubsystem))
  (|CallParentFunction)
  (Utilities|IsValid _eventsubsystem
    (:Is%20Valid
      (EventDispatchers|UnbindEventfromOnEvent (Class|EventSubsystem|GetEventChannel _eventsubsystem "/Game/Lyzandred/Blueprints/Events/DA_KeyCollectedChannel.DA_KeyCollectedChannel") (delegate Custom|OnEvent)))))