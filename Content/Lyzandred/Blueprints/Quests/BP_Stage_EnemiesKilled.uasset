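; Quest stage that completes once the player has killed the required number of each enemy type.
; While listening, it binds to the kill-enemies event channel from the event subsystem, resetting its tally first and unbinding on Clear.
; Each kill payload increments a count keyed by the enemy class's TypeId.
; The stage completes when every count exactly equals its EnemiesToKill target, rather than meeting or exceeding it.
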(event Custom|OnEvent
  (params (EventTag :type Name) (Sender :type Object%20Object%20Reference) (Payload :type Event%20Payload%20Object%20Object%20Reference))
  (switch name EventTag
    (:KillEnemy
      (bind _asbp_kill_enemy_payload (Utilities|Casting|CastToBP_KillEnemyPayload Payload))
      (if (Utilities|Map|Contains (Variables|Default|GetEnemiesKilled) (.TypeId (Utilities|GetClassDefaults (Variables|/Game/Lyzandred/Blueprints/Events/BP_KillEnemyPayload.BP_KillEnemyPayload_C|GetEnemyType _asbp_kill_enemy_payload))))
        (bind _result (Math|Integer|IncrementInt (.Value (Utilities|Map|Find (Variables|Default|GetEnemiesKilled) (.TypeId (Utilities|GetClassDefaults (Variables|/Game/Lyzandred/Blueprints/Events/BP_KillEnemyPayload.BP_KillEnemyPayload_C|GetEnemyType _asbp_kill_enemy_payload))))))
          (:%20%20
            (Utilities|Map|Add (Variables|Default|GetEnemiesKilled) (.TypeId (Utilities|GetClassDefaults (Variables|/Game/Lyzandred/Blueprints/Events/BP_KillEnemyPayload.BP_KillEnemyPayload_C|GetEnemyType _asbp_kill_enemy_payload))) _result)))
        (else
          (Utilities|Map|Add (Variables|Default|GetEnemiesKilled) (.TypeId (Utilities|GetClassDefaults (Variables|/Game/Lyzandred/Blueprints/Events/BP_KillEnemyPayload.BP_KillEnemyPayload_C|GetEnemyType _asbp_kill_enemy_payload))) 1)))
      (if (CallFunction|CheckifEnoughEnemiesKilled)
        (Class|QuestStage|CompleteStage)))))

(event EventListenforCompletion
  (bind _eventsubsystem (Variables|Default|GetEventSubsystem))
  (Utilities|Map|Clear (Variables|Default|GetEnemiesKilled))
  (Utilities|IsValid _eventsubsystem
    (:Is%20Valid
      (EventDispatchers|BindEventtoOnEvent (Class|EventSubsystem|GetEventChannel _eventsubsystem "/Game/Lyzandred/Blueprints/Events/DA_KillEnemiesEventChannel.DA_KillEnemiesEventChannel") (EventDispatchers|CreateEvent :!event Custom|OnEvent)))))

(event EventClear
  (bind _eventsubsystem (Variables|Default|GetEventSubsystem))
  (|CallParentFunction)
  (Utilities|IsValid _eventsubsystem
    (:Is%20Valid
      (EventDispatchers|UnbindEventfromOnEvent (Class|EventSubsystem|GetEventChannel _eventsubsystem "/Game/Lyzandred/Blueprints/Events/DA_KillEnemiesEventChannel.DA_KillEnemiesEventChannel") (delegate Custom|OnEvent)))))

(fn CheckifEnoughEnemiesKilled
  (bind _keys (Utilities|Map|Keys (Variables|QuestSubsystem|GetEnemiesToKill)))
  (bind _array_element (Utilities|Array|ForEachLoopwithBreak _keys :!label _label)
    (:LoopBody
      (if (not (== (.Value (Utilities|Map|Find (Variables|Default|GetEnemiesKilled) (.TypeId (Utilities|GetClassDefaults _array_element)))) (.Value (Utilities|Map|Find (Variables|QuestSubsystem|GetEnemiesToKill) _array_element))))
        (LocalVariables|SetAreEqual false)
        (goto _label Break)))
    (:Completed
      (return (LocalVariables|GetAreEqual)))))