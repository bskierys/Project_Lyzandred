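; Quest Blueprint that activates when an area with a matching name is entered.
; It listens on the enter-area event channel from the event subsystem and casts each payload to the enter-area payload type.
; When the payload's AreaName equals its own AreaName it activates the quest.
; Clear runs the parent cleanup and unbinds from the channel.
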(event Custom|OnAreaEvent
  (params (EventTag :type Name) (Sender :type Object%20Object%20Reference) (Payload :type Event%20Payload%20Object%20Object%20Reference))
  (bind _asbp_enter_area_payload (Utilities|Casting|CastToBP_EnterAreaPayload Payload))
  (if (== (Variables|/Game/Lyzandred/Blueprints/Events/BP_EnterAreaPayload.BP_EnterAreaPayload_C|GetAreaName _asbp_enter_area_payload) (Variables|QuestSubsystem|GetAreaName))
    (Class|Quest|ActivateQuest)))

(event EventListenforActivation
  (bind _eventsubsystem (Variables|Default|GetEventSubsystem))
  (Utilities|IsValid _eventsubsystem
    (:Is%20Valid
      (EventDispatchers|BindEventtoOnEvent (Class|EventSubsystem|GetEventChannel _eventsubsystem "/Game/Lyzandred/Blueprints/Events/DA_EnterAreaEventChannel.DA_EnterAreaEventChannel") (EventDispatchers|CreateEvent :!event Custom|OnAreaEvent)))))

(event EventClear
  (bind _eventsubsystem (Variables|Default|GetEventSubsystem))
  (|CallParentFunction)
  (Utilities|IsValid _eventsubsystem
    (:Is%20Valid
      (EventDispatchers|UnbindEventfromOnEvent (Class|EventSubsystem|GetEventChannel _eventsubsystem "/Game/Lyzandred/Blueprints/Events/DA_EnterAreaEventChannel.DA_EnterAreaEventChannel") (delegate Custom|OnAreaEvent)))))