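; Tutorial prompt for the Sage in the main level that changes its message as story progress is made.
; On BeginPlay it casts the game state to Lyz_GameState and binds to its key-changed event.
; When the "EvilBook" key becomes true, it sets the prompt widget to the Sage's second main-level dialogue entry.
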(event Custom|OnKeyChanged
  (params (Key :type Name) (Value :type Boolean))
  (if (and (== Key "EvilBook") Value)
    (Default|SetMessage (Variables|Default|GetPromptWidget) "Dialogue_MainLevel_Sage2")))

(event EventBeginPlay
  (|CallParentFunction)
  (bind _aslyz_game_state (Utilities|Casting|CastToLyz_GameState (Game|GetGameState)))
  (bind _output_get (Variables|Default|SetGameStateRef _aslyz_game_state))
  (EventDispatchers|BindEventtoOnKeyChanged _output_get (EventDispatchers|CreateEvent :!event Custom|OnKeyChanged)))

(fn ConstructionScript
  (|CallParentFunction))