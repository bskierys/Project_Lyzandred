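; Static mesh prop Blueprint that shows a pulsing colored glow through an overlay material while IsGlowActive is set.
; BeginPlay creates a dynamic instance of GlowingMaterial, applies GlowColor, sets it as the overlay and starts a looping timer as a custom tick.
; While active, the tick feeds a sine pulse from ComputeGlowValue into GlowIntensity, and zeroes it once on deactivation.
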(event Custom|OnCustomTick
  (bind _bisglowactive (Variables|Glow|GetbIsGlowActive))
  (if _bisglowactive
    (Variables|Default|SetbPreviousGlowActive _bisglowactive)
    ;[0.15 0.15 0.15 0.5] Set Glow Intensity for this tick
    (Variables|Default|SetRunningTime (+ (Variables|Default|GetRunningTime) (Variables|Default|GetDeltaTime)))
    (Rendering|Material|SetScalarParameterValue (Variables|Default|GetDynamicOverlay) "GlowIntensity" (CallFunction|ComputeGlowValue) :!class /Script/Engine.MaterialInstanceDynamic)
    (else
      ;[0.15 0.15 0.15 0.5] Reset the glow when deactivated in this tick
      (if (Variables|Default|GetbPreviousGlowActive)
        (Variables|Default|SetbPreviousGlowActive false)
        (Rendering|Material|SetScalarParameterValue (Variables|Default|GetDynamicOverlay) "GlowIntensity" 0.0 :!class /Script/Engine.MaterialInstanceDynamic)))))

(event EventBeginPlay
  (bind _returnvalue (Rendering|Material|CreateDynamicMaterialInstance (Variables|Glow|GetGlowingMaterial) "None" "None" :!class /Script/Engine.KismetMaterialLibrary))
  (bind _output_get (Variables|Default|SetDynamicOverlay _returnvalue))
  (Rendering|Material|SetVectorParameterValue _output_get "GlowColor" (Variables|Glow|GetGlowColor) :!class /Script/Engine.MaterialInstanceDynamic)
  (Rendering|Material|SetOverlayMaterial _output_get :!class /Script/Engine.MeshComponent)
  (Utilities|Time|SetTimerbyEvent (EventDispatchers|CreateEvent :!event Custom|OnCustomTick) (Variables|Default|GetDeltaTime) true true))

(fn ComputeGlowValue
  (return (+ (* (/ (+ (Math|Trig|Sin(Radians) (* (Variables|Default|GetRunningTime) (Variables|Glow|GetGlowSpeed))) 1.0) 2.0) (Variables|Glow|GetPulseStrength)) (Variables|Glow|GetBaseGlow))))