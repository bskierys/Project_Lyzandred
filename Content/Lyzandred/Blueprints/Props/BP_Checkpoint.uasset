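; Checkpoint prop that sets the player's respawn location when the player pawn enters it, with chimes and a glowing mesh showing active state.
; Overlap, gated by a DoOnce that resets on exit, activates it and sends its offset transform to BP_Lyz_PlayerController.
; Each checkpoint listens to the controller's respawn-change event and deactivates on a non-matching transform, without checking whether it was active.
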(event Custom|OnCheckpointActivated
  ;[0.15 0.15 0.15 0.5] Activation / Deactivation Logic
  (Audio|PlaySoundatLocation "/Game/Lyzandred/Assets/SFX/SFX_Chime_02A.SFX_Chime_02A" (Transformation|GetActorLocation) "0, 0, 0" 1.0 1.0 0.0 0 0 0 0)
  (bind _output_get (Variables|Default|SetbIsActive true))
  (Variables|/Game/Lyzandred/Blueprints/Props/BP_GlowingStatickMesh.BP_GlowingStatickMesh_C|SetbIsGlowActive (Variables|Default|GetBP_GlowingStatickMesh) _output_get)
  (Default|SetRespawnLocation (Variables|Default|GetLyzPlayerController) (CallFunction|GetCheckpointTransform)))

(event Custom|OnCheckpoinDeactivated
  ;[0.15 0.15 0.15 0.5] Activation / Deactivation Logic
  (Audio|PlaySoundatLocation "/Game/Lyzandred/Assets/SFX/SFX_Chime_04A.SFX_Chime_04A" (Transformation|GetActorLocation) "0, 0, 0" 1.0 1.0 0.0 0 0 0 0)
  (bind _output_get (Variables|Default|SetbIsActive false))
  (Variables|/Game/Lyzandred/Blueprints/Props/BP_GlowingStatickMesh.BP_GlowingStatickMesh_C|SetbIsGlowActive (Variables|Default|GetBP_GlowingStatickMesh) _output_get))

(event Custom|OnRespawnLocationChanged
  (params (RespawnLocation :type Transform))
  ;[0.15 0.15 0.15 0.5] Deactivate when other activated
  (if (not (== RespawnLocation (CallFunction|GetCheckpointTransform)))
    (CallFunction|OnCheckpoinDeactivated)))

(event EventBeginPlay
  (Utilities|FlowControl|Sequence
    (:then_0
      ;[0.15 0.15 0.15 0.5] Initialize Glow Animation
      (Variables|/Game/Lyzandred/Blueprints/Props/BP_GlowingStatickMesh.BP_GlowingStatickMesh_C|SetbIsGlowActive (Variables|Default|GetBP_GlowingStatickMesh) (Variables|Default|GetbIsActive)))
    (:then_1
      (bind _output_get (Variables|Default|SetLyzPlayerController (.AsBP%20Lyz%20Player%20Controller (Utilities|Casting|CastToBP_Lyz_PlayerController (Game|GetPlayerController 0)))))
      (EventDispatchers|BindEventtoOnRespawnLocationChanged _output_get (EventDispatchers|CreateEvent :!event Custom|OnRespawnLocationChanged)))))

(event Collision|EventActorBeginOverlap
  (params (OtherActor :type Actor%20Object%20Reference))
  ;[0.15 0.15 0.15 0.5] When to Activate / Deactivate chackpoint
  (if (Class|LyzCharacterLibrary|CheckifCurrentPlayerPawn OtherActor)
    (Utilities|FlowControl|DoOnce false
      (:Completed
        (if (not (Variables|Default|GetbIsActive))
          (CallFunction|OnCheckpointActivated))))))

(event Collision|EventActorEndOverlap
  (params (OtherActor :type Actor%20Object%20Reference))
  ;[0.15 0.15 0.15 0.5] When to Activate / Deactivate chackpoint
  (if (Class|LyzCharacterLibrary|CheckifCurrentPlayerPawn OtherActor)
    (Utilities|FlowControl|DoOnce false) ; enters at Reset
  ))

(event EventEndPlay
  (params (EndPlayReason :type EEndPlayReason%20Enum :default "Destroyed"))
  ;[0.15 0.15 0.15 0.5] Deactivate when other activated
  (Utilities|IsValid (Variables|Default|GetLyzPlayerController)
    (:Is%20Valid
      (EventDispatchers|UnbindEventfromOnRespawnLocationChanged (Variables|Default|GetLyzPlayerController) (delegate Custom|OnRespawnLocationChanged)))))

(fn ConstructionScript)

(fn GetCheckpointTransform
  (return (Math|Transform|MakeTransform (+ (Transformation|GetActorLocation) (Variables|Default|GetSpawnOffset)) (Transformation|GetActorRotation) (Transformation|GetActorScale3D))))