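; BP_InteractableComponent is a widget component that gives its owning actor an interaction prompt and an interactable state.
; On BeginPlay it caches its WBP_InteractPrompt widget, sets the text and hides it.
; It tracks requested visibility separately from the interactable flag, showing the prompt only when both are true, so re-enabling reveals a requested prompt immediately.
; Changing the flag also messages the owner, and the text can be updated at runtime.
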(event Custom|SetInteractWidgetVisibility
  (params (bVisible :type Boolean))
  ;[0.15 0.15 0.15 0.5] Whow the widget only if Enabled
  (bind _output_get (Variables|Default|SetbShouldBeShown bVisible))
  (if _output_get
    (if (Variables|Default|GetbInteractable)
      (CallFunction|InternalSetVisible true))
    (else
      (CallFunction|InternalSetVisible false))))

(event Custom|SetInteractable
  (params (bIsEnabled :type Boolean))
  ;[0.15 0.15 0.15 0.5] When enabled check if should be shown. If so, show immidiately.
  (bind _output_get (Variables|Default|SetbInteractable bIsEnabled))
  (Class|LyzInteractableInterface|OnInteractableChanged(Message) (Components|GetOwner) _output_get)
  (if (Variables|Default|GetbShouldBeShown)
    (CallFunction|InternalSetVisible (Variables|Default|GetbInteractable))))

(event EventBeginPlay
  (|CallParentFunction)
  ;[0.15 0.15 0.15 0.5] Setup Interaction Widget
  (bind _aswbp_interact_prompt (Utilities|Casting|CastToWBP_InteractPrompt (UserInterface|GetUserWidgetObject)))
  (bind _output_get (Variables|Default|SetInteractWidget _aswbp_interact_prompt))
  (Default|SetText _output_get (Variables|Default|GetText))
  (CallFunction|InternalSetVisible false))

(fn IsInteractable
  (return (Variables|Default|GetbInteractable)))

(fn InternalSetVisible
  (params (bVisible :type Boolean))
  (if bVisible
    (Variables|/Script/UMG.Widget|SetVisibility (Variables|Default|GetInteractWidget) "Visible")
    (else
      (Variables|/Script/UMG.Widget|SetVisibility (Variables|Default|GetInteractWidget) "Hidden"))))

(fn UpdateText
  (params (Text :type Text))
  (bind _output_get (Variables|Default|SetText Text))
  (Default|SetText (Variables|Default|GetInteractWidget) _output_get))