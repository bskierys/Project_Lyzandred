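; Character component that lets its owning character detect and use interactable props.
; Capsule overlaps toggle each prop's interact widget and toast the combined reasons from any locked components through the game mode.
; The interact input sends an interface message to every overlapping interactable actor, passing the owner and a normalized direction from object to character.
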(event Custom|OnBeginOverlap
  (params (OverlappedComponent :type Primitive%20Component%20Object%20Reference) (OtherActor :type Actor%20Object%20Reference) (OtherComp :type Primitive%20Component%20Object%20Reference) (OtherBodyIndex :type Integer) (bFromSweep :type Boolean) (SweepResult :type Hit%20Result%20Structure%20%28by%20ref%29))
  ;[0.15 0.15 0.15 0.5] Showing and Hiding Widget
  (bind _interactablecomponent (CallFunction|ExtractInteractableComponent OtherActor))
  (Utilities|IsValid _interactablecomponent
    (:Is%20Valid
      (Default|SetInteractWidgetVisibility _interactablecomponent true)
      ;[0.15 0.15 0.15 0.5] If not interactable, show the message why
      (bind _components (CallFunction|ExtractUnlockableLockedComponents OtherActor))
      (bind _message (CallFunction|CreateLockedText _components))
      (if (not (Utilities|Text|TextIsEmpty _message))
        (Default|DisplayToast (Variables|Default|GetGameModeRef) _message)))))

(event Custom|OnEndOverlap
  (params (OverlappedComponent :type Primitive%20Component%20Object%20Reference) (OtherActor :type Actor%20Object%20Reference) (OtherComp :type Primitive%20Component%20Object%20Reference) (OtherBodyIndex :type Integer))
  ;[0.15 0.15 0.15 0.5] Showing and Hiding Widget
  (bind _interactablecomponent (CallFunction|ExtractInteractableComponent OtherActor))
  (Utilities|IsValid _interactablecomponent
    (:Is%20Valid
      (Default|SetInteractWidgetVisibility _interactablecomponent false))))

(event Input|EnhancedActionEvents|EnhancedInputActionIA_Interact
  (params (ActionValue :type Boolean) (ElapsedSeconds :type Float%20%28double-precision%29) (TriggeredSeconds :type Float%20%28double-precision%29) (InputAction :type Input%20Action%20Object%20Reference :default "/Game/Lyzandred/Input/IA_Interact.IA_Interact"))
  ;[0.15 0.15 0.15 0.5] Object Interaction
  (bind _array_element (Utilities|Array|ForEachLoopwithBreak (Collision|GetOverlappingActors (Variables|Default|GetCharacter%20Ref) 0 :!class /Script/Engine.Actor))
    (:LoopBody
      (if (Utilities|DoesObjectImplementInterface _array_element "/Script/Project_Lyzandred.Lyz_InteractableInterface")
        (Class|LyzInteractableInterface|Interact(Message) _array_element (Components|GetOwner) (Math|Vector|Normalize (- (Transformation|GetActorLocation (Variables|Default|GetCharacter%20Ref)) (Transformation|GetActorLocation _array_element))))))))

(event EventBeginPlay
  ;[0.15 0.15 0.15 0.5] Initialization
  (bind _output_get (Variables|Default|SetCharacter%20Ref (.AsCharacter (Utilities|Casting|CastToCharacter (Components|GetOwner)))))
  (Collision|BindEventtoOnComponentBeginOverlap (Variables|/Script/Engine.Character|GetCapsuleComponent _output_get) (EventDispatchers|CreateEvent :!event Custom|OnBeginOverlap))
  (Collision|BindEventtoOnComponentEndOverlap (Variables|/Script/Engine.Character|GetCapsuleComponent _output_get) (EventDispatchers|CreateEvent :!event Custom|OnEndOverlap))
  (Variables|Default|SetGameModeRef (.AsBP%20Lyz%20Game%20Mode (Utilities|Casting|CastToBP_Lyz_GameMode (Game|GetGameMode)))))

(fn CreateLockedText
  (params (Components :type Array%20of%20BP%20Unlockable%20Component%20Object%20References))
  (for _array_element Components
    (bind _message (Default|CreateWhyLockedMessage _array_element))
    (Utilities|Array|Add (LocalVariables|GetTextArray) _message))
  (bind _message_2 (CallFunction|ArrayOfTextstoText (LocalVariables|GetTextArray)))
  (return _message_2))