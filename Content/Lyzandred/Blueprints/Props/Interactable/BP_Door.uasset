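; Interactable door that swings open on player interaction and can also be opened or closed through switch events.
; A timeline drives the door's yaw, with swing direction picked from the dot product of the interaction direction and the actor's right vector.
; Interaction is disabled while open.
; With AutoClose set, leaving the trigger box starts a timer that closes the door, and re-entering pauses that timer.
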(event OnComponentEndOverlap(Box)
  (params (OverlappedComponent :type Primitive%20Component%20Object%20Reference) (OtherActor :type Actor%20Object%20Reference) (OtherComp :type Primitive%20Component%20Object%20Reference) (OtherBodyIndex :type Integer))
  ;[0.15 0.15 0.15 0.5] Auto-closing the door
  (if (Math|Boolean|ANDBoolean (Class|LyzCharacterLibrary|CheckifCurrentPlayerPawn OtherActor) (Variables|Default|GetisOpen) (Variables|Default|GetbAutoClose))
    (bind _returnvalue (Utilities|Time|SetTimerbyEvent (delegate Custom|CloseAgain) (Variables|Default|GetCloseAfter)))
    (Variables|Default|SetCloseTimer _returnvalue)))

(event OnComponentBeginOverlap(Box)
  (params (OverlappedComponent :type Primitive%20Component%20Object%20Reference) (OtherActor :type Actor%20Object%20Reference) (OtherComp :type Primitive%20Component%20Object%20Reference) (OtherBodyIndex :type Integer) (bFromSweep :type Boolean) (SweepResult :type Hit%20Result%20Structure%20%28by%20ref%29))
  ;[0.15 0.15 0.15 0.5] Auto-closing the door
  (if (and (Class|LyzCharacterLibrary|CheckifCurrentPlayerPawn OtherActor) (Utilities|Time|IsValidTimerHandle (Variables|Default|GetCloseTimer)))
    (Utilities|Time|PauseTimerbyHandle (Variables|Default|GetCloseTimer))))

(event Custom|OpenOrCloseDoor
  (params (DirectionVector :type Vector%20%28by%20ref%29))
  ;[0.15 0.15 0.15 0.5] Open Animation
  (if (Variables|Default|GetisOpen)
    (bind _open (Timeline|Door%20Open%20Timeline Reverse)
      (:Update
        (Transformation|SetRelativeRotation (Variables|Default|GetDoor) (Math|Rotator|MakeRotator 0.0 0.0 (* _open (Variables|Default|GetSwingAngle) (Variables|Default|GetSwingDirection))) false false))
      (:Finished
        (Variables|Default|SetisOpen (not (Variables|Default|GetisOpen)))
        (Default|SetInteractable (Variables|Default|GetInteractableComponent) (not (Variables|Default|GetisOpen)))))
    (else
      (bind _swingdirectionmultiplier (CallFunction|ComputeSwingDirection DirectionVector))
      (Variables|Default|SetSwingDirection _swingdirectionmultiplier)
      (Timeline|Door%20Open%20Timeline PlayFromStart))))

(event Custom|CloseAgain
  ;[0.15 0.15 0.15 0.5] Auto-closing the door
  (Class|LyzSwitchableInterface|SwitchOff))

(event EventSwitchon
  ;[0.15 0.15 0.15 0.5] Open / Close without Interaction
  (if (not (Variables|Default|GetisOpen))
    (CallFunction|OpenorCloseDoor "0, 0, 0")))

(event EventInteract
  (params (Caller :type Actor%20Object%20Reference) (DirectionVector :type Vector :default "0, 0, 0"))
  ;[0.15 0.15 0.15 0.5] Interaction
  (if (Default|IsInteractable (Variables|Default|GetInteractableComponent))
    (if (not (Variables|Default|GetisOpen))
      (CallFunction|OpenorCloseDoor DirectionVector))))

(event EventBeginPlay
  ;[0.15 0.15 0.15 0.5] Setup Interaction Widget
  (Default|UpdateText (Variables|Default|GetInteractableComponent) (Variables|Default|GetOpenText)))

(event EventSwitchOff
  ;[0.15 0.15 0.15 0.5] Open / Close without Interaction
  (if (Variables|Default|GetisOpen)
    (CallFunction|OpenorCloseDoor "0, 0, 0")))

(fn ConstructionScript)

(fn UpdateWidgetText
  (params (Widget :type WBP%20Interact%20Prompt%20Object%20Reference))
  (Default|SetText Widget (Variables|Default|GetOpenText)))

(fn ComputeSwingDirection
  (params (InteractionDirection :type Vector))
  (if (> (Math|Vector|DotProduct InteractionDirection (Transformation|GetActorRightVector)) 0.0)
    (return -1)
    (else
      (return 1))))