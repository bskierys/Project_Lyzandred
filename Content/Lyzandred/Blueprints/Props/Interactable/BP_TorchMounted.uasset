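; Wall-mounted torch prop whose flame can be switched on and off through events that toggle the Fire component and its children.
; The construction script hides the fire when unlit; when lit, it scales the light's intensity and radius by a strength multiplier.
; Lit torches can also flicker through a dynamic light function material with randomized speed on a Stationary light.
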(event EventSwitchOff
  (if (Variables|Default|GetbIsLit)
    (Rendering|SetVisibility (Variables|Default|GetFire) false true)
    (Variables|Default|SetbIsLit false)))

(event EventSwitchon
  (if (not (Variables|Default|GetbIsLit))
    (Rendering|SetVisibility (Variables|Default|GetFire) true true)
    (Variables|Default|SetbIsLit true)))

(fn ConstructionScript
  ;[0.15 0.15 0.15 0.5] Flame on/off
  (if (Variables|Default|GetbIsLit)
    (Utilities|FlowControl|Sequence
      (:then_0
        ;[0.15 0.15 0.15 0.5] Flickering Light
        (if (Variables|Default|GetShouldFlicker)
          (Transformation|SetMobility (Variables|Default|GetFlameLight) "Stationary")
          (bind _returnvalue (Rendering|Material|CreateDynamicMaterialInstance "/Game/Lyzandred/Assets/Materials/M_FlickeringLight.M_FlickeringLight" "None" "None" :!class /Script/Engine.KismetMaterialLibrary))
          (Variables|Default|SetFlickeringLightMaterial _returnvalue)
          (Rendering|Material|SetScalarParameterValue (Variables|Default|GetFlickeringLightMaterial) "Speed" (Math|Random|RandomFloatinRange 2.0 5.0) :!class /Script/Engine.MaterialInstanceDynamic)
          (Rendering|Material|SetScalarParameterValue (Variables|Default|GetFlickeringLightMaterial) "MinIntensity" 0.8 :!class /Script/Engine.MaterialInstanceDynamic)
          (Rendering|Material|SetScalarParameterValue (Variables|Default|GetFlickeringLightMaterial) "MaxIntensity" 1.0 :!class /Script/Engine.MaterialInstanceDynamic)
          (Rendering|Components|Light|SetLightFunctionMaterial (Variables|Default|GetFlameLight) (Variables|Default|GetFlickeringLightMaterial))))
      (:then_1
        ;[0.15 0.15 0.15 0.5] Change Strength of light
        (Rendering|Components|Light|SetIntensity (Variables|Default|GetFlameLight) (* (Variables|/Script/Engine.LightComponentBase|GetIntensity (Variables|Default|GetFlameLight)) (Variables|Default|GetStrengthMultiplier)))
        (Rendering|Lighting|SetAttenuationRadius (Variables|Default|GetFlameLight) (* (Variables|/Script/Engine.LocalLightComponent|GetAttenuationRadius (Variables|Default|GetFlameLight)) (Variables|Default|GetStrengthMultiplier)))))
    (else
      (Rendering|SetVisibility (Variables|Default|GetFire) false true))))