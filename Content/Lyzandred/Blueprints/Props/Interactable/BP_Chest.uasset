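; Interactable treasure chest that opens once, swinging its lid and playing a sound, and reveals a ring of coins.
; The construction script configures a child-actor BP_CircleCoinSpawner with hidden coins and attaches it to the chest so coins follow moving parents.
; Interact disables further interaction and runs the OpenLid timeline, which rotates the lid and triggers the spawner's coin animation on both update and finish.
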(event EventInteract
  (params (Caller :type Actor%20Object%20Reference) (DirectionVector :type Vector :default "0, 0, 0"))
  ;[0.15 0.15 0.15 0.5] Interaction
  (if (Default|IsInteractable (Variables|Default|GetInteractableComponent))
    (Utilities|FlowControl|DoOnce false
      (:Completed
        (Variables|Default|SetbIsOpen true)
        (Default|SetInteractable (Variables|Default|GetInteractableComponent) false)
        (Utilities|FlowControl|Sequence
          (:then_0
            ;;[0.15 0.15 0.15 0.5] Open Chast Lid
            (bind _lid_float_rotation (Timeline|Open%20Lid Play)
              (:Update
                (Transformation|SetRelativeRotation (Variables|Default|Getchest_lid) (Math|Rotator|MakeRotator (* _lid_float_rotation -1e+01) 0.0 0.0) false false)
                ;;[0.15 0.15 0.15 0.5] Animate Coin Spawn when animation is over
                (Utilities|IsValid (Variables|Default|GetCoinCircleSpawn)
                  (:Is%20Valid
                    _)))
              (:Finished
                _))
            (Class|LyzCoinSpawner|AnimateCoinSpawn (Variables|Default|GetCoinCircleSpawn)))
          (:then_1
            ;;[0.15 0.15 0.15 0.5] Play Sound
            (Audio|PlaySoundatLocation "/Game/Lyzandred/Assets/SFX/SFX_ChestOpen.SFX_ChestOpen" (Transformation|GetActorLocation) "0, 0, 0" 1.0 1.0 0.0 0 0 0 0)))))))

(fn ConstructionScript
  ;[0.15 0.15 0.15 0.5] Spawn Circle of Coins around but hide it until character interacts
  (bind _asbp_circle_coin_spawner (Utilities|Casting|CastToBP_CircleCoinSpawner (Variables|/Script/Engine.ChildActorComponent|GetChildActor (Variables|Default|GetCoinCircle))))
  (Variables|Default|SetCoinCircleSpawn _asbp_circle_coin_spawner)
  (Variables|/Script/Project_Lyzandred.Lyz_CoinSpawner|SetCoins (Variables|Default|GetCoinCircleSpawn) (Variables|Default|GetCoins))
  (Variables|/Script/Project_Lyzandred.Lyz_CoinSpawner|SetbCoinsVisible (Variables|Default|GetCoinCircleSpawn) false)
  (Variables|/Script/Project_Lyzandred.Lyz_CircleCoinSpawner|SetCoinSpawnRadius (Variables|Default|GetCoinCircleSpawn) (Variables|Default|GetCoinSpawnRadius))
  ;[0.15 0.15 0.15 0.5] Attach to self to keep coins while rooted to platforms
  (Transformation|AttachActorToActor (Variables|Default|GetCoinCircleSpawn) self "None" "KeepWorld" "KeepWorld" "KeepWorld" true))