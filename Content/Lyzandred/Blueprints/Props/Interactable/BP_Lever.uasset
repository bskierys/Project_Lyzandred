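; Interactable lever prop that toggles on or off, swinging its handle with a timeline that blocks re-toggling while it plays.
; Each change writes the state to its ActivatedKey in the Lyz game state and drives a glow overlay on two indicator lights, provided the key is valid.
; An optional countdown through the timer subsystem shows a HUD timer and switches the lever back off when it expires.
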(event Custom|OnActivationChanged
  (Utilities|IsValid (Variables|Default|GetActivatedKey)
    (:Is%20Valid
      (Class|LyzGameState|SetKey (Class|LyzGameStateLibrary|GetLyzGameState) (Variables|Default|GetActivatedKey) (Variables|Default|GetbIsActivated))
      (if (Variables|Default|GetbIsActivated)
        (Rendering|Material|SetScalarParameterValue (Variables|Default|GetGlowOverlay) "GlowIntensity" 2e+01 :!class /Script/Engine.MaterialInstanceDynamic)
        (if (> (Variables|Default|GetDeactivateAfterTime) 0.0)
          (Class|TimerSubsystem|StartCountdown (Subsystems|GetTimerSubsystem) (Variables|Default|GetDeactivateAfterTime) (EventDispatchers|CreateEvent :!event Custom|OnTimerFinished))
          (Class|BPIHud|SetTimerVisibility(Message) (HUD|GetHUD (Game|GetPlayerController 0)) "Visible"))
        (else
          (Rendering|Material|SetScalarParameterValue (Variables|Default|GetGlowOverlay) "GlowIntensity" 0.0 :!class /Script/Engine.MaterialInstanceDynamic))))))

(event Custom|OnTimerFinished
  (CallFunction|SwitchOff)
  (Utilities|FlowControl|Delay 3.0)
  (if (not (Class|TimerSubsystem|IsRunning (Subsystems|GetTimerSubsystem)))
    (Class|BPIHud|SetTimerVisibility(Message) (HUD|GetHUD (Game|GetPlayerController 0)) "Hidden")))

(event EventSwitchOff
  (if (Variables|Default|GetbIsActivated)
    (if (not (Variables|Default|GetbIsAnimRunning))
      (Variables|Default|SetbIsActivated (not (Variables|Default|GetbIsActivated)))
      (CallFunction|OnActivationChanged)
      (Variables|Default|SetbIsAnimRunning true)
      (bind _lever (Timeline|Timeline PlayFromStart)
        (:Update
          (Transformation|SetRelativeRotation (Variables|Default|GetSM_LeverHandle) (Math|Rotator|MakeRotator 0.0 (* (- (* _lever 6e+01) 3e+01) (select (Variables|Default|GetbIsActivated) 1 -1)) 0.0) false false))
        (:Finished
          (Variables|Default|SetbIsAnimRunning false))))))

(event EventInteract
  (params (Caller :type Actor%20Object%20Reference) (DirectionVector :type Vector :default "0, 0, 0"))
  ;[0.15 0.15 0.15 0.5] Interaction
  (if (Variables|Default|GetbIsActivated)
    (CallFunction|SwitchOff)
    (else
      (CallFunction|Switchon))))

(event EventSwitchon
  (if (not (Variables|Default|GetbIsActivated))
    (if (not (Variables|Default|GetbIsAnimRunning))
      (Variables|Default|SetbIsActivated (not (Variables|Default|GetbIsActivated)))
      (CallFunction|OnActivationChanged)
      (Variables|Default|SetbIsAnimRunning true)
      (bind _lever (Timeline|Timeline PlayFromStart)
        (:Update
          (Transformation|SetRelativeRotation (Variables|Default|GetSM_LeverHandle) (Math|Rotator|MakeRotator 0.0 (* (- (* _lever 6e+01) 3e+01) (select (Variables|Default|GetbIsActivated) 1 -1)) 0.0) false false))
        (:Finished
          (Variables|Default|SetbIsAnimRunning false))))))

(event EventBeginPlay
  (bind _returnvalue (Rendering|Material|CreateDynamicMaterialInstance "/Game/Lyzandred/Assets/Materials/MI_GlowOverlayDefault.MI_GlowOverlayDefault" "None" "None" :!class /Script/Engine.KismetMaterialLibrary))
  (Variables|Default|SetGlowOverlay _returnvalue)
  (Rendering|Material|SetOverlayMaterial (Variables|Default|GetActivateLight1) (Variables|Default|GetGlowOverlay) :!class /Script/Engine.MeshComponent)
  (Rendering|Material|SetOverlayMaterial (Variables|Default|GetActivateLight2) (Variables|Default|GetGlowOverlay) :!class /Script/Engine.MeshComponent)
  (CallFunction|OnActivationChanged))

(fn ConstructionScript)

(fn GetInteractable
  (return false))