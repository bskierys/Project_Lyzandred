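; BP_TutorialPrompt is a trigger prop that shows a tutorial dialogue message while the player stands inside its box.
; On BeginPlay it creates a WBP_DialogueMessage widget and fills it with the configurable title and message.
; Box overlap by player pawn 0 adds the widget to the viewport through a DoOnce, and leaving removes it and resets the gate so it can show again.
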(event OnComponentBeginOverlap(Box)
  (params (OverlappedComponent :type Primitive%20Component%20Object%20Reference) (OtherActor :type Actor%20Object%20Reference) (OtherComp :type Primitive%20Component%20Object%20Reference) (OtherBodyIndex :type Integer) (bFromSweep :type Boolean) (SweepResult :type Hit%20Result%20Structure%20%28by%20ref%29))
  (if (== OtherActor (Game|Player|GetPlayerPawn 0))
    (Utilities|FlowControl|DoOnce false
      (:Completed
        (UserInterface|Viewport|AddtoViewport (Variables|Default|GetPromptWidget) 0)))))

(event OnComponentEndOverlap(Box)
  (params (OverlappedComponent :type Primitive%20Component%20Object%20Reference) (OtherActor :type Actor%20Object%20Reference) (OtherComp :type Primitive%20Component%20Object%20Reference) (OtherBodyIndex :type Integer))
  (if (== OtherActor (Game|Player|GetPlayerPawn 0))
    (Widget|RemovefromParent (Variables|Default|GetPromptWidget))
    (Utilities|FlowControl|DoOnce false) ; enters at Reset
  ))

(event EventBeginPlay
  (bind _returnvalue (UserInterface|CreateWidget "/Game/Lyzandred/Blueprints/Widgets/WBP_DialogueMessage.WBP_DialogueMessage_C"))
  (Variables|Default|SetPromptWidget _returnvalue)
  (Default|SetTitle (Variables|Default|GetPromptWidget) (Variables|Default|GetPromptTitle))
  (Default|SetMessage (Variables|Default|GetPromptWidget) (Variables|Default|GetPromptMessage)))

(fn ConstructionScript)