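; BP_RotatingPlatform is a magic prop platform whose rotation can be paused, resumed and reversed through events.
; BeginPlay caches the RotatingMovement component's initial rotation rate.
; Pause zeroes the rate, Play restores the cached rate, and Reverse toggles a flag that sets its sign.
; Play ignores that flag, so it always resumes in the original direction, while Reverse also restarts a paused platform.
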(event EventBeginPlay
  (bind _rotatingmovement (Variables|Default|GetRotatingMovement))
  (Utilities|IsValid _rotatingmovement
    (:Is%20Valid
      (Variables|Default|SetRotationRate (Variables|/Script/Engine.RotatingMovementComponent|GetRotationRate _rotatingmovement)))))

(event EventPauseMovement
  (bind _rotatingmovement (Variables|Default|GetRotatingMovement))
  (Utilities|IsValid _rotatingmovement
    (:Is%20Valid
      (Variables|/Script/Engine.RotatingMovementComponent|SetRotationRate _rotatingmovement "0, 0, 0"))))

(event EventPlayMovement
  (bind _rotatingmovement (Variables|Default|GetRotatingMovement))
  (Utilities|IsValid _rotatingmovement
    (:Is%20Valid
      (Variables|/Script/Engine.RotatingMovementComponent|SetRotationRate _rotatingmovement (Variables|Default|GetRotationRate)))))

(event EventReverseMovement
  (bind _rotatingmovement (Variables|Default|GetRotatingMovement))
  (Variables|Default|SetbIsReversed (not (Variables|Default|GetbIsReversed)))
  (Utilities|IsValid _rotatingmovement
    (:Is%20Valid
      (Variables|/Script/Engine.RotatingMovementComponent|SetRotationRate _rotatingmovement (* (Variables|Default|GetRotationRate) (Math|Float|SelectFloat -1.0 1.0 (Variables|Default|GetbIsReversed)))))))

(fn ConstructionScript)