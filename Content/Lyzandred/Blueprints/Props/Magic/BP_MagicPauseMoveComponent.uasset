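; Magic-interaction component that pauses and resumes movement of its owning prop in the game.
; Toggling with magic flips a moving flag, seeded from an initial setting at begin play, and sends play or pause movement messages to the owner.
; Leaving the mage form always restarts movement and marks the prop as moving.
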(event EventTogglewithMagic
  (bind _returnvalue (Components|GetOwner))
  (Variables|Default|SetbIsMoving (not (Variables|Default|GetbIsMoving)))
  (if (Variables|Default|GetbIsMoving)
    (Class|LyzMovingPropInterface|PlayMovement(Message) _returnvalue)
    (else
      (Class|LyzMovingPropInterface|PauseMovement(Message) _returnvalue))))

(event EventOnfromMagicForm
  (|CallParentFunction)
  ;[0.15 0.15 0.15 0.5] When Form changed from mage, start movement again
  (Class|LyzMovingPropInterface|PlayMovement(Message) (Components|GetOwner))
  (Variables|Default|SetbIsMoving true))

(event EventBeginPlay
  (|CallParentFunction)
  (Variables|Default|SetbIsMoving (Variables|Default|GetbIsInitiallyMoving)))