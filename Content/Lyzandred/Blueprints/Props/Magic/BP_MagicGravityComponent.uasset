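; BP_MagicGravityComponent is a magic component that lets magic switch gravity and physics simulation on or off for a prop.
; Activate, deactivate and toggle events set GravityEnabled, and RefreshGravityState applies it to every entry in PrimitiveComponents.
; BeginPlay applies InitialGravityEnabled after a zero-length delay.
; Entering magic form reapplies the current state, while leaving it restores the initial one.
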(event EventBeginPlay
  (|CallParentFunction)
  (Utilities|FlowControl|Delay 0.0)
  (Variables|Magic|SetbGravityEnabled (Variables|Magic|GetbInitialGravityEnabled))
  (CallFunction|RefreshGravityState))

(event EventActivatewithMagic
  (Variables|Magic|SetbGravityEnabled true)
  (CallFunction|RefreshGravityState))

(event EventDeactivatewithMagic
  (Variables|Magic|SetbGravityEnabled false)
  (CallFunction|RefreshGravityState))

(event EventTogglewithMagic
  (Variables|Magic|SetbGravityEnabled (not (Variables|Magic|GetbGravityEnabled)))
  (CallFunction|RefreshGravityState))

(event EventOnfromMagicForm
  (|CallParentFunction)
  (Variables|Magic|SetbGravityEnabled (Variables|Magic|GetbInitialGravityEnabled))
  (CallFunction|RefreshGravityState))

(event EventOntoMagicForm
  (|CallParentFunction)
  (Variables|Magic|SetbGravityEnabled (Variables|Magic|GetbGravityEnabled))
  (CallFunction|RefreshGravityState))

(fn RefreshGravityState
  (bind _bgravityenabled (Variables|Magic|GetbGravityEnabled))
  (for _array_element (Variables|Default|GetPrimitiveComponents)
    (Physics|SetEnableGravity (.Component (Utilities|Struct|BreakPrimitiveComponentInfo _array_element)) _bgravityenabled)
    (Physics|SetSimulatePhysics (.Component (Utilities|Struct|BreakPrimitiveComponentInfo _array_element)) _bgravityenabled)))