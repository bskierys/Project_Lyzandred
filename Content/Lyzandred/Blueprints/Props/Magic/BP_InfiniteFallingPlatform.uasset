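; Prop platform that falls endlessly between a lower and an upper portal, tumbling at a random rotation rate.
; The construction script derives respawn heights from fall distance, margin and mesh height, then positions the platform and upper portal.
; While playing, Tick moves the platform vertically and teleports it back to the start when it passes the end.
; Movement interface events play, pause or reverse it, with reversal swapping endpoints and negating speed.
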(event EventBeginPlay
  (bind _maxrotation (Variables|Default|GetMaxRotation))
  (bind _minrotation (Variables|Default|GetMinRotation))
  ;[0.15 0.15 0.15 0.5] Randomize Platform Rotation to simulate falling
  (Variables|Default|SetFallRotation (Math|Rotator|MakeRotator (Math|Random|RandomFloatinRange _minrotation _maxrotation) (Math|Random|RandomFloatinRange _minrotation _maxrotation) (Math|Random|RandomFloatinRange _minrotation _maxrotation)))
  ;[0.15 0.15 0.15 0.5] Set Start/End based on is the movement Reversed
  (CallFunction|RecomputeStartEnd))

(event EventPlayMovement
  ;[0.15 0.15 0.15 0.5] Movement Control Interface Methods
  (Variables|Default|SetbIsPlaying true))

(event EventTick
  (params (DeltaSeconds :type Float%20%28single-precision%29))
  (bind _returnvalue (Transformation|GetActorLocation))
  (bind _returnvalue_2 (Transformation|GetActorLocation))
  ;[0.15 0.15 0.15 0.5] Moving the platform on Tick Event
  (if (Variables|Default|GetbIsPlaying)
    ;;[0.15 0.15 0.15 0.5] Tick can be uneaven. Compute proper speed based on delta seconds.
    (Variables|Default|SetTickMoveDelta (* DeltaSeconds (Variables|Default|GetSpeed)))
    ;;[0.15 0.15 0.15 0.5] Recompute Start/End and Speed only if something changed
    (if (Variables|Default|GetbHasReverseChanged)
      (CallFunction|RecomputeStartEnd)
      (Variables|Default|SetbHasReverseChanged false))
    (if (or (and (< (Variables|Default|GetCurrentZ) (Variables|Default|GetEndZLocation)) (not (Variables|Default|GetbIsReversed))) (and (> (Variables|Default|GetCurrentZ) (Variables|Default|GetEndZLocation)) (Variables|Default|GetbIsReversed)))
      ;;[0.15 0.15 0.15 0.5] Teleport to beginning
      (Transformation|SetWorldLocation (Variables|Default|GetPlatform) (Math|Vector|MakeVector (.x _returnvalue) (.y _returnvalue) (Variables|Default|GetStartZLocation)) false true)
      (Variables|Default|SetCurrentZ (Variables|Default|GetStartZLocation))
      (else
        ;;[0.15 0.15 0.15 0.5] Move Platform
        (bind _output_get (Variables|Default|SetCurrentZ (+ (Variables|Default|GetCurrentZ) (Variables|Default|GetTickMoveDelta))))
        (Transformation|SetWorldLocation (Variables|Default|GetPlatform) (Math|Vector|MakeVector (.x _returnvalue_2) (.y _returnvalue_2) _output_get) false true)
        (Transformation|AddLocalRotation (Variables|Default|GetPlatform) (Variables|Default|GetFallRotation) false false)))))

(event EventPauseMovement
  ;[0.15 0.15 0.15 0.5] Movement Control Interface Methods
  (Variables|Default|SetbIsPlaying false))

(event EventReverseMovement
  ;[0.15 0.15 0.15 0.5] Movement Control Interface Methods
  (Variables|Default|SetbIsReversed (not (Variables|Default|GetbIsReversed)))
  (Variables|Default|SetbHasReverseChanged true))

(fn ConstructionScript
  (bind _returnvalue (Transformation|GetActorLocation))
  (bind _returnvalue_2 (Transformation|GetActorLocation))
  (Variables|Default|SetZSize (CallFunction|GetMeshZSize (Variables|Default|GetPlatform)))
  ;[0.15 0.15 0.15 0.5] Apply Margin to Lower Respawn Location to avoid collision with floor
  (Variables|Default|SetLowerZLocation (+ (.z (Transformation|GetActorLocation)) (Variables|Default|GetMargin)))
  ;[0.15 0.15 0.15 0.5] Compute Upper Respawn Location Based on Fall Distance
  (Variables|Default|SetUpperZLocation (Utilities|Operators|Subtract (+ (Variables|Default|GetFallDistance) (Variables|Default|GetLowerZLocation)) (Variables|Default|GetZSize) (Variables|Default|GetMargin)))
  ;[0.15 0.15 0.15 0.5] Set Starting position
  (bind _output_get (Variables|Default|SetCurrentZ (- (Variables|Default|GetUpperZLocation) (Variables|Default|GetFallOffset))))
  ;[0.15 0.15 0.15 0.5] Place Platform Mesh in Starting Location
  (Transformation|SetWorldLocation (Variables|Default|GetPlatform) (Math|Vector|MakeVector (.x _returnvalue_2) (.y _returnvalue_2) _output_get) false false)
  ;[0.15 0.15 0.15 0.5] Adjust only Upper Portal. Lower should be fixed on 0,0
  (Transformation|SetWorldLocation (Variables|Default|GetPortalUp) (Math|Vector|MakeVector (.x _returnvalue) (.y _returnvalue) (+ (Variables|Default|GetUpperZLocation) (/ (Variables|Default|GetZSize) 2.0))) false false))

(fn GetMeshZSize
  (params (MeshComponent :type Static%20Mesh%20Component%20Object%20Reference))
  (return (* (.z (.boxextent (StaticMesh|GetBounds (Variables|/Script/Engine.StaticMeshComponent|GetStaticMesh MeshComponent)))) (.z (Variables|/Script/Engine.SceneComponent|GetRelativeScale3D MeshComponent)) 2.0)))

(fn RecomputeStartEnd
  (Variables|Default|SetSpeed (* (Variables|Default|GetSpeed) -1.0))
  (if (Variables|Default|GetbIsReversed)
    (Variables|Default|SetStartZLocation (Variables|Default|GetLowerZLocation))
    (Variables|Default|SetEndZLocation (Variables|Default|GetUpperZLocation))
    (else
      (Variables|Default|SetStartZLocation (Variables|Default|GetUpperZLocation))
      (Variables|Default|SetEndZLocation (Variables|Default|GetLowerZLocation)))))