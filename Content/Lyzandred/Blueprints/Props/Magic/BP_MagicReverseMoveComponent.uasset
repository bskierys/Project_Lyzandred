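; BP_MagicReverseMoveComponent is a magic component that lets the mage form reverse the movement of the prop it is attached to.
; Each magic toggle flips IsReversed and sends ReverseMovementMessage to the owning actor, which handles the movement itself.
; Leaving magic form runs the parent logic, then, if still reversed, sends the message again and clears the flag so movement returns to normal.
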(event EventTogglewithMagic
  (Variables|Default|SetbIsReversed (not (Variables|Default|GetbIsReversed)))
  (Class|LyzMovingPropInterface|ReverseMovement(Message) (Components|GetOwner)))

(event EventOnfromMagicForm
  (|CallParentFunction)
  (if (Variables|Default|GetbIsReversed)
    ;[0.15 0.15 0.15 0.5] When Form changed from mage, start movement again
    (Class|LyzMovingPropInterface|ReverseMovement(Message) (Components|GetOwner))
    (Variables|Default|SetbIsReversed false)))