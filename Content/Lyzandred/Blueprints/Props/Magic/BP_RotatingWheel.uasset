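; BP_RotatingWheel is a magic prop that spins through a rotating movement component and can be paused, resumed or reversed.
; On BeginPlay it caches the component's rotation rate, then pausing zeroes that rate and playing restores it in the forward direction.
; Reversing flips the sign of the cached rate and only works while unpaused.
; SwitchOff and Switchon events map to pause and play.
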(event EventBeginPlay
  (bind _rotatingmovement (Variables|Default|GetRotatingMovement))
  (Utilities|IsValid _rotatingmovement
    (:Is%20Valid
      (Variables|Default|SetRotationRate (Variables|/Script/Engine.RotatingMovementComponent|GetRotationRate _rotatingmovement)))))

(event EventSwitchOff
  (CallFunction|PauseMovement))

(event EventSwitchon
  (CallFunction|PlayMovement))

(event EventPauseMovement
  (bind _rotatingmovement (Variables|Default|GetRotatingMovement))
  (Utilities|IsValid _rotatingmovement
    (:Is%20Valid
      (Variables|/Script/Engine.RotatingMovementComponent|SetRotationRate _rotatingmovement "0, 0, 0")
      (Variables|Default|SetbIsPaused true))))

(event EventPlayMovement
  (bind _rotatingmovement (Variables|Default|GetRotatingMovement))
  (Utilities|IsValid _rotatingmovement
    (:Is%20Valid
      (Variables|/Script/Engine.RotatingMovementComponent|SetRotationRate _rotatingmovement (Variables|Default|GetRotationRate))
      (Variables|Default|SetbIsReversed false)
      (Variables|Default|SetbIsPaused false))))

(event EventReverseMovement
  (bind _rotatingmovement (Variables|Default|GetRotatingMovement))
  (if (not (Variables|Default|GetbIsPaused))
    (Variables|Default|SetbIsReversed (not (Variables|Default|GetbIsReversed)))
    (Utilities|IsValid _rotatingmovement
      (:Is%20Valid
        (Variables|/Script/Engine.RotatingMovementComponent|SetRotationRate _rotatingmovement (* (Variables|Default|GetRotationRate) (Math|Float|SelectFloat -1.0 1.0 (Variables|Default|GetbIsReversed))))))))

(fn ConstructionScript)