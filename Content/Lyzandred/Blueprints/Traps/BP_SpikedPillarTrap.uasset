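; Trap actor for a spiked pillar that moves along a path while spinning and kills the player character on contact.
; The construction script feeds its InterpToMovement component a configurable duration and two relative control points, from the origin to MoveToPosition.
; On BeginPlay, a Rotation timeline drives the capsule's yaw.
; Capsule overlaps pass the other actor to KillIfLyzCharacter.
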(event OnComponentBeginOverlap(Capsule)
  (params (OverlappedComponent :type Primitive%20Component%20Object%20Reference) (OtherActor :type Actor%20Object%20Reference) (OtherComp :type Primitive%20Component%20Object%20Reference) (OtherBodyIndex :type Integer) (bFromSweep :type Boolean) (SweepResult :type Hit%20Result%20Structure%20%28by%20ref%29))
  (Class|LyzTrap|KillifLyzCharacter OtherActor))

(event EventBeginPlay
  (bind _rotationz (Timeline|Rotation Play)
    (:Update
      (Transformation|SetRelativeRotation (Variables|Default|GetCapsule) (Math|Rotator|MakeRotator 0.0 0.0 _rotationz) false false))))

(fn ConstructionScript
  (Variables|/Script/Engine.InterpToMovementComponent|SetDuration (Variables|Default|GetInterpToMovement) (Variables|Default|GetMovementDuration))
  (Class|InterptoMovementComponent|AddControlPointPosition (Variables|Default|GetInterpToMovement) "0, 0, 0" true)
  (Class|InterptoMovementComponent|AddControlPointPosition (Variables|Default|GetInterpToMovement) (Variables|Default|GetMoveToPosition) true))