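; BP_Lava is a lava trap actor whose own logic only fits an optional rect light to the placed size.
; The construction script runs the parent's, then derives light source size, intensity and attenuation radius from root world scale, since rect lights do not scale themselves.
; Padding shrinks the source dimensions, and disabling HasLightEffect hides the light to save cost in open areas.
; The event graph is empty.
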(event Collision|EventActorBeginOverlap
  (params (OtherActor :type Actor%20Object%20Reference)))

(event EventTick
  (params (DeltaSeconds :type Float%20%28single-precision%29)))

(fn ConstructionScript
  (bind _defaultsceneroot (Variables|Default|GetDefaultSceneRoot))
  (bind _defaultsceneroot_2 (Variables|Default|GetDefaultSceneRoot))
  (bind _returnvalue (Transformation|GetWorldScale _defaultsceneroot_2))
  (bind _returnvalue_2 (Transformation|GetWorldScale _defaultsceneroot))
  (|CallParentFunction)
  (if (Variables|Default|GetbHasLightEffect)
    ;[0.15 0.15 0.15 0.5] Rect Light can't be scaled, so we need to scale it ourselves
    (Class|RectLightComponent|SetSourceHeight (Variables|Default|GetRectLight) (- (* (.x _returnvalue_2) (Variables|/Script/Engine.RectLightComponent|GetSourceHeight (Variables|Default|GetRectLight))) (Variables|Default|GetLightPadding)))
    (Class|RectLightComponent|SetSourceWidth (Variables|Default|GetRectLight) (- (* (.y _returnvalue_2) (Variables|/Script/Engine.RectLightComponent|GetSourceWidth (Variables|Default|GetRectLight))) (Variables|Default|GetLightPadding)))
    (Rendering|Components|Light|SetIntensity (Variables|Default|GetRectLight) (* (.x (Transformation|GetWorldScale (Variables|Default|GetDefaultSceneRoot))) (Variables|/Script/Engine.LightComponentBase|GetIntensity (Variables|Default|GetRectLight))))
    (Rendering|Lighting|SetAttenuationRadius (Variables|Default|GetRectLight) (* (Variables|/Script/Engine.LocalLightComponent|GetAttenuationRadius (Variables|Default|GetRectLight)) (Math|Float|Min(Float) (.x _returnvalue) (.y _returnvalue))))
    (else
      ;[0.15 0.15 0.15 0.5] Turn off the light for open areas for optimisation
      (Rendering|SetVisibility (Variables|Default|GetRectLight) false false))))