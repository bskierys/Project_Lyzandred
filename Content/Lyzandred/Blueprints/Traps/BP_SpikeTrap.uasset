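; Spike trap Blueprint that calls KillPawn on any actor that begins overlapping its box collision.
; The construction script builds a centered grid of spike meshes from configurable row, column and spacing values, using an Instanced Static Mesh component.
; It also sizes the box collision to the grid plus padding, so the kill area follows the spike layout.
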(event OnComponentBeginOverlap(Box)
  (params (OverlappedComponent :type Primitive%20Component%20Object%20Reference) (OtherActor :type Actor%20Object%20Reference) (OtherComp :type Primitive%20Component%20Object%20Reference) (OtherBodyIndex :type Integer) (bFromSweep :type Boolean) (SweepResult :type Hit%20Result%20Structure%20%28by%20ref%29))
  (Class|LyzTrap|KillPawn OtherActor))

(fn ConstructionScript
  ;[0.15 0.15 0.15 0.5] Compute Center point
  (LocalVariables|SetCenterX (* (- (Variables|Default|GetRowSpikes) 1) (Variables|Default|GetGapBetweenSpikes) 0.5))
  (LocalVariables|SetCenterY (* (- (Variables|Default|GetColumnsSpikes) 1) (Variables|Default|GetGapBetweenSpikes) 0.5))
  ;[0.15 0.15 0.15 0.5] Created Instanced Static Mesh
  (bind _returnvalue (AddComponent|AddInstancedStaticMeshComponent false))
  (bind _output_get (LocalVariables|SetSpikeMeshInstance _returnvalue))
  (Components|StaticMesh|SetStaticMesh _output_get "/Game/Lyzandred/Assets/Meshes/SM_Spike.SM_Spike")
  ;[0.15 0.15 0.15 0.5] Extend Box Collision for Spikes
  (Components|Box|SetBoxExtent (Variables|Default|GetBox) (Math|Vector|MakeVector (+ (LocalVariables|GetCenterX) (LocalVariables|GetBoxCollisionPadding)) (+ (LocalVariables|GetCenterY) (LocalVariables|GetBoxCollisionPadding)) (LocalVariables|GetBoxCollisionPadding)) true)
  ;[0.15 0.15 0.15 0.5] Loop over row and columns to create a spike array
  (for _index (range 0 (- (Variables|Default|GetColumnsSpikes) 1))
    (for _index_2 (range 0 (- (Variables|Default|GetRowSpikes) 1))
      (Components|InstancedStaticMesh|AddInstance (LocalVariables|GetSpikeMeshInstance) (Math|Transform|MakeTransform (Math|Vector|MakeVector (- (* _index_2 (Variables|Default|GetGapBetweenSpikes)) (LocalVariables|GetCenterX)) (- (* _index (Variables|Default|GetGapBetweenSpikes)) (LocalVariables|GetCenterY)) 0.0) "0, 0, 0" "1.000000,1.000000,1.000000") false))))