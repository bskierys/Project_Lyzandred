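; Area trigger volume that announces when the current player pawn enters a named area.
; On overlap by that pawn, it builds an enter-area payload carrying its AreaName and sends it on the DA_EnterAreaEventChannel through the event subsystem.
; The construction script sizes the box from AreaSize and shows AreaName on a text component.
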(event EventBeginPlay)

(event Collision|EventActorBeginOverlap
  (params (OtherActor :type Actor%20Object%20Reference))
  (if (Class|LyzCharacterLibrary|CheckifCurrentPlayerPawn OtherActor)
    (bind _returnvalue (Game|ConstructObjectfromClass "/Game/Lyzandred/Blueprints/Events/BP_EnterAreaPayload.BP_EnterAreaPayload_C"))
    (Variables|/Game/Lyzandred/Blueprints/Events/BP_EnterAreaPayload.BP_EnterAreaPayload_C|SetAreaName _returnvalue (Variables|Default|GetAreaName))
    (Class|EventSubsystem|SendEvent (Subsystems|GetEventSubsystem) "/Game/Lyzandred/Blueprints/Events/DA_EnterAreaEventChannel.DA_EnterAreaEventChannel" "None" self _returnvalue)))

(event EventTick
  (params (DeltaSeconds :type Float%20%28single-precision%29)))

(fn ConstructionScript
  (Components|Box|SetBoxExtent (Variables|Default|GetBox) (Variables|Default|GetAreaSize) true)
  (Rendering|Components|TextRender|SetText (Variables|Default|GetNameText) (Utilities|Text|ToText(Name) (Variables|Default|GetAreaName))))