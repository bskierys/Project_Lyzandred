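; BP_EventTestActor2 is a test listener actor for the event channel system, using DA_TestEventChannel.
; It binds to the channel through the EventSubsystem on BeginPlay and unbinds OnTestChannelEvent on EndPlay.
; When an event arrives, it casts the payload to BP_TestPayloadObject and prints its TestString, ignoring other payload types.
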(event Custom|OnTestChannelEvent
  (params (Event :type Event%20Channel%20Object%20Reference) (EventTag :type Name) (Sender :type Object%20Object%20Reference) (Payload :type Event%20Payload%20Object%20Object%20Reference))
  (bind _asbp_test_payload_object (Utilities|Casting|CastToBP_TestPayloadObject Payload))
  (Development|PrintString (Utilities|String|Append "Test Event Received. Payload: " (Variables|/Game/Lyzandred/Blueprints/Events/BP_TestPayloadObject.BP_TestPayloadObject_C|GetTestString _asbp_test_payload_object))))

(event EventBeginPlay
  (EventDispatchers|BindEventtoOnEvent (Class|EventSubsystem|GetEventChannel (Subsystems|GetEventSubsystem) "/Game/Lyzandred/Blueprints/Events/DA_TestEventChannel.DA_TestEventChannel") (EventDispatchers|CreateEvent :!event Custom|OnTestChannelEvent)))

(event EventEndPlay
  (params (EndPlayReason :type EEndPlayReason%20Enum :default "Destroyed"))
  (EventDispatchers|UnbindEventfromOnEvent (Class|EventSubsystem|GetEventChannel (Subsystems|GetEventSubsystem) "/Game/Lyzandred/Blueprints/Events/DA_TestEventChannel.DA_TestEventChannel") (delegate Custom|OnTestChannelEvent)))

(fn ConstructionScript)