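; Player controller for Lyzandred that handles input mapping setup, pause menu toggling, and character death and respawn.
; On death it unpossesses the pawn, shows a game-over widget after a short delay, then spawns and possesses a same-class replacement once the fade-in finishes, destroying the old pawn.
; The respawn transform defaults to the first PlayerStart found; its setter broadcasts changes through a dispatcher.
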(event Custom|On%20Game%20Over%20Screen%20Loaded
  (bind _currentplayerpawn (Variables|Default|GetCurrentPlayerPawn))
  ;[0.15 0.15 0.15 0.5] Character Death
  ;;[0.15 0.15 0.15 0.5] When animation finishes, Spawn new Character, posses and destroy an old one
  ;;;[0.15 0.15 0.15 0.5] Spawn Pawn of same class as killedat the PlayerStart location, and possess it.
  (bind _returnvalue (Game|SpawnActorfromClass (Variables|Default|GetCurrentPawnClass) (Variables|Default|GetRespawnLocation) "AlwaysSpawn" "MultiplyWithRoot" 0 0))
  (Pawn|Possess _returnvalue)
  ;;;[0.15 0.15 0.15 0.5] Destroy the old pawn
  (Utilities|IsValid _currentplayerpawn
    (:Is%20Valid
      (Actor|DestroyActor _currentplayerpawn))))

(event Input|EnhancedActionEvents|EnhancedInputActionIA_Pause
  (params (ActionValue :type Boolean) (ElapsedSeconds :type Float%20%28double-precision%29) (TriggeredSeconds :type Float%20%28double-precision%29) (InputAction :type Input%20Action%20Object%20Reference :default "/Game/Lyzandred/Input/IA_Pause.IA_Pause"))
  ;[0.15 0.15 0.15 0.5] Pause Game
  (:Started
    (if (Game|IsGamePaused)
      (Game|SetGamePaused false)
      ;;[0.15 0.15 0.15 0.5] Add or Remove Pause Menu Widget
      (Utilities|IsValid (Variables|Default|GetPauseMenuWidget)
        (:Is%20Valid
          (Widget|RemovefromParent (Variables|Default|GetPauseMenuWidget))))
      (else
        (Game|SetGamePaused true)
        (bind _returnvalue (UserInterface|CreateWidget "/Game/Lyzandred/Blueprints/Widgets/WBP_PauseMenu.WBP_PauseMenu_C"))
        (bind _output_get (Variables|Default|SetPauseMenuWidget _returnvalue))
        (UserInterface|Viewport|AddtoViewport _output_get 0)))))

(event EventBeginPlay
  (Utilities|FlowControl|Sequence
    (:then_0
      ;[0.15 0.15 0.15 0.5] Set Enhanced Input Mapping
      (Input|AddMappingContext (PlayerController|LocalPlayerSubsystems|GetEnhancedInputLocalPlayerSubsystem) "/Game/Lyzandred/Input/IMC_Default.IMC_Default" 0 "(bIgnoreAllPressedKeysUntilRelease=True,bForceImmediately=False,bNotifyUserSettings=False)")
      (Input|AddMappingContext (PlayerController|LocalPlayerSubsystems|GetEnhancedInputLocalPlayerSubsystem) "/Game/Lyzandred/Input/IMC_PauseMenu.IMC_PauseMenu" 0 "(bIgnoreAllPressedKeysUntilRelease=True,bForceImmediately=False,bNotifyUserSettings=False)")
      ;[0.15 0.15 0.15 0.5] Remember Game State to reset state on death
      (bind _aslyz_game_state (Utilities|Casting|CastToLyz_GameState (Game|GetGameState)))
      (Variables|Default|SetGameStateRef _aslyz_game_state))
    (:then_1
      ;[0.15 0.15 0.15 0.5] Initial Respawn Location - default if no checkpoint active
      (bind _outactors (Actor|GetAllActorsOfClass "/Script/Engine.PlayerStart"))
      (Variables|Default|SetRespawnLocation (Transformation|GetActorTransform (Utilities|Array|Get(acopy) _outactors))))))

(event EventEndPlay
  (params (EndPlayReason :type EEndPlayReason%20Enum :default "Destroyed"))
  (EventDispatchers|UnbindallEventsfromOnRespawnLocationChanged))

(event EventKillCurrentCharacter
  (bind _returnvalue (Game|Player|GetPlayerPawn 0))
  ;[0.15 0.15 0.15 0.5] Character Death
  ;;[0.15 0.15 0.15 0.5] First, unposses pawn, wait a little then show widget with animation
  (Variables|Default|SetCurrentPlayerPawn _returnvalue)
  (Variables|Default|SetCurrentPawnClass (Utilities|GetClass _returnvalue))
  (Pawn|UnPossess)
  ;;;[0.15 0.15 0.15 0.5] Delay before showin widget to watch death animation
  (Utilities|FlowControl|Delay 0.5)
  (bind _returnvalue_2 (UserInterface|CreateWidget "/Game/Lyzandred/Blueprints/Widgets/WBP_GameOver.WBP_GameOver_C"))
  (bind _output_get (Variables|Default|SetGameOverWidget _returnvalue_2))
  (UserInterface|Viewport|AddtoViewport _output_get 0)
  (Class|UserWidget|BindtoAnimationFinished (Variables|Default|GetGameOverWidget) (Variables|/Game/Lyzandred/Blueprints/Widgets/WBP_GameOver.WBP_GameOver_C|GetFadeIn (Variables|Default|GetGameOverWidget)) (EventDispatchers|CreateEvent :!event Custom|On%20Game%20Over%20Screen%20Loaded)))

(event EventPossess
  (params (PossessedPawn :type Pawn%20Object%20Reference))
  ;[0.15 0.15 0.15 0.5] Pawn initialization
  (bind _aslyz_triform_character (Utilities|Casting|CastToLyz_TriformCharacter PossessedPawn))
  (Variables|/Script/Project_Lyzandred.Lyz_TriformCharacter|SetControllerReference _aslyz_triform_character self))

(fn ConstructionScript)

(fn SetRespawnLocation
  (params (NewLocation :type Transform))
  (bind _output_get (Variables|Default|SetRespawnLocation NewLocation))
  (Default|CallOnRespawnLocationChanged _output_get))

(fn GetRespawnLocation
  (return (Variables|Default|GetRespawnLocation)))