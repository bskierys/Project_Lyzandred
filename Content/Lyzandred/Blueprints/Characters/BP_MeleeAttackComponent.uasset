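; Melee attack component that detects weapon hits on killable actors during an attack window.
; Opening the window stores the weapon and starts a fast looping timer, while closing it clears both.
; The overlap check damages the first non-owner actor implementing Lyz_KillableInterface and calls OnAttackHit.
; A DoOnce reset after a short delay throttles the check, whether or not it hits.
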(event Custom|AttackWindowOpen
  (params (Weapon :type Primitive%20Component%20Object%20Reference))
  (Variables|Default|SetWeapon Weapon)
  (Variables|Default|SetbIsAttackActive true)
  (bind _returnvalue (Utilities|Time|SetTimerbyEvent (EventDispatchers|CreateEvent :!event Custom|CheckDamagedActors) 0.01 true true))
  (Variables|Default|SetDamagedActorsTimer _returnvalue))

(event Custom|AttackWindowClose
  (Variables|Default|SetWeapon 0)
  (Variables|Default|SetbIsAttackActive false)
  (Utilities|Time|InvalidateTimerHandle (Variables|Default|GetDamagedActorsTimer)))

(event Custom|CheckDamagedActors
  (if (Variables|Default|GetbIsAttackActive)
    (Utilities|FlowControl|DoOnce false :!label _label
      (:Completed
        (bind _array_element (Utilities|Array|ForEachLoopwithBreak (Collision|GetOverlappingActors (Variables|Default|GetWeapon) 0 :!class /Script/Engine.PrimitiveComponent) :!label _label_2)
          (:LoopBody
            (if (!= _array_element (Components|GetOwner))
              (if (Utilities|DoesObjectImplementInterface _array_element "/Script/Project_Lyzandred.Lyz_KillableInterface")
                (Utilities|FlowControl|Sequence
                  (:then_0
                    (Class|LyzKillableInterface|Damage(Message) _array_element)
                    (Default|CallOnAttackHit _array_element))
                  (:then_1
                    (goto _label_2 Break))))))
          (:Completed
            (Utilities|FlowControl|Delay 0.5)
            (goto _label Reset)))))))