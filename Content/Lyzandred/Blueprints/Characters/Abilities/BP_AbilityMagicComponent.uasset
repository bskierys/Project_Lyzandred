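; Magic ability component that plays a casting montage and reveals or toggles nearby magical objects.
; On the montage's Cast notify it spawns a BP_RevealWave at an offset relative to the owner's facing and attaches it to the owner.
; A sphere overlap around the owner then finds actors tagged Magic and calls the toggle message on their first component implementing Lyz_MagicTogglableInterface.
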(event EventActivateAbility
  (bind _returnvalue (Components|GetOwner))
  (bind _returnvalue_2 (Components|GetOwner))
  (bind _returnvalue_3 (Transformation|GetActorTransform _returnvalue_2))
  (|CallParentFunction)
  (bind _notifyname (Animation|Montage|PlayMontage (Variables|/Script/Engine.Character|GetMesh (Variables|Default|GetCharacterRef)) "/Game/Lyzandred/Assets/Animations/Adventurers/Mage/AM_CastingSpell.AM_CastingSpell")
    (:OnNotifyBegin
      (if (== _notifyname "Cast")
        ;[0.15 0.15 0.15 0.5] Spawn Sphere animation
        (bind _returnvalue_4 (Game|SpawnActorfromClass "/Game/Lyzandred/Blueprints/Characters/Abilities/BP_RevealWave.BP_RevealWave_C" (Math|Transform|MakeTransform (CallFunction|ComputeCastLocation) (.rotation _returnvalue_3) (.scale _returnvalue_3)) "AlwaysSpawn" "MultiplyWithRoot" 0 (Variables|Default|GetActivationRadius) (Variables|Default|GetAnimationDuration) 0))
        (Transformation|AttachActorToActor _returnvalue_4 (Components|GetOwner) "None" "KeepWorld" "KeepWorld" "KeepWorld" true)
        ;[0.15 0.15 0.15 0.5] Activate all Actors in the Radius that hasa magical component
        (bind _outactors (Collision|SphereOverlapActors (Transformation|GetActorLocation _returnvalue) (* (Variables|Default|GetActivationRadius) (Variables|Default|GetAnimationSphereRadius)) (Variables|Default|GetDetectionTypes) 0 (Utilities|Array|MakeArray _returnvalue)))
        (for _array_element _outactors
          (if (Actor|ActorHasTag _array_element "Magic")
            (if (> (Utilities|Array|Length (Class|Actor|GetComponentsbyInterface _array_element "/Script/Project_Lyzandred.Lyz_MagicTogglableInterface")) 0)
              (Class|LyzMagicTogglableInterface|TogglewithMagic(Message) (Utilities|Array|Get(acopy) (Class|Actor|GetComponentsbyInterface _array_element "/Script/Project_Lyzandred.Lyz_MagicTogglableInterface"))))))))))

(fn ComputeCastLocation
  (bind _returnvalue (Components|GetOwner))
  (bind _castspawnoffset (Variables|Default|GetCastSpawnOffset))
  (bind _castspawnoffset_2 (Variables|Default|GetCastSpawnOffset))
  (bind _returnvalue_2 (Transformation|GetActorForwardVector _returnvalue))
  (bind _returnvalue_3 (Transformation|GetActorRightVector _returnvalue))
  (bind _returnvalue_4 (Math|Vector|Normalize _returnvalue_3))
  (bind _returnvalue_5 (Math|Vector|Normalize _returnvalue_2))
  (bind _returnvalue_6 (* _returnvalue_4 (.y _castspawnoffset_2)))
  (bind _returnvalue_7 (* _returnvalue_5 (.x _castspawnoffset)))
  (bind _returnvalue_8 (+ _returnvalue_7 _returnvalue_6))
  (return (+ (.location (Transformation|GetActorTransform _returnvalue)) (Math|Vector|MakeVector (.x _returnvalue_8) (.y _returnvalue_8) (.z (Variables|Default|GetCastSpawnOffset))))))