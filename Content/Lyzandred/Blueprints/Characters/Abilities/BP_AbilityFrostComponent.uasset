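; Frost ability component for a character, handling the camera and light changes that accompany the ability switching on and off.
; Activation runs the parent logic, then animates the owning character's camera to a configured location offset and shows its light.
; Deactivation also runs the parent logic, then plays the same camera offset in reverse and hides the light.
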(event EventActivateAbility
  (bind _characterref (Variables|Default|GetCharacterRef))
  (|CallParentFunction)
  (Class|LyzTriformCharacter|AnimateCameraOffset _characterref (Variables|Default|GetCameraLocationOffset) false)
  (Class|LyzTriformCharacter|SetLightVisibility _characterref true))

(event EventDeactivateAbility
  (bind _characterref (Variables|Default|GetCharacterRef))
  (|CallParentFunction)
  (Class|LyzTriformCharacter|AnimateCameraOffset _characterref (Variables|Default|GetCameraLocationOffset) true)
  (Class|LyzTriformCharacter|SetLightVisibility _characterref false))