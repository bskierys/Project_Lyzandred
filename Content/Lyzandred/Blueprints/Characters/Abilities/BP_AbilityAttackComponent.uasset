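; Ability component that gives a character a sword attack on the ground and a ground pound in the air, blocked during wall slide.
; Montage notifies open and close the melee component's hit window, or end the mid-air freeze with a downward launch.
; Landing adds impact feedback and a cooldown before restoring control, while Tick exits the pound early if the character moves upward.
; Sword hits trigger sound, rumble, camera shake and noise.
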(event Custom|OnCharacterLanded
  (params (Hit :type Hit%20Result%20Structure%20%28by%20ref%29))
  (bind _returnvalue (Components|GetOwner))
  (bind _returnvalue_2 (Transformation|GetActorLocation _returnvalue))
  ;[0.15 0.15 0.15 0.5] Character Landed
  ;;[0.15 0.15 0.15 0.5] Guard against invoking to often
  (if (and (Variables|Default|GetbIsGroundPounding) (not (Variables|Default|GetbHasLanded)))
    (Variables|Default|SetbHasLanded true)
    ;;[0.15 0.15 0.15 0.5] Special Effects
    (CameraShakes|StartCameraShake (Variables|/Script/Engine.PlayerController|GetPlayerCameraManager (Game|GetPlayerController 0)) "/Game/Lyzandred/Blueprints/Effects/BP_GroundPoundShake.BP_GroundPoundShake_C" 1.0 "CameraLocal" "0, 0, 0")
    (ForceFeedback|SpawnForceFeedbackatLocation "/Game/Lyzandred/Input/FF_GroundPound.FF_GroundPound" (Transformation|GetActorLocation (Components|GetOwner)) "0, 0, 0" false 1.0 0.0 0)
    (Audio|PlaySoundatLocation "/Game/Lyzandred/Assets/SFX/SFX_Thud1.SFX_Thud1" _returnvalue_2 "0, 0, 0" 1.0 1.0 0.0 0 0 0 0)
    (Class|Pawn|PawnMakeNoise (Variables|Default|GetCharacterRef) 1e+02 _returnvalue_2 true 0)
    ;;[0.15 0.15 0.15 0.5] Short Delay to have a little penalty for powerfull effect
    (Utilities|FlowControl|Delay (Variables|Default|GetGroundPoundCooldown))
    (CallFunction|ExitGroundPound)))

(event Custom|ExitGroundPound
  (bind _characterref (Variables|Default|GetCharacterRef))
  ;[0.15 0.15 0.15 0.5] Reset Ground Pound values regardless how we landed
  (Variables|Default|SetbIsGroundPounding false)
  (Class|LyzAbilityComponent|BroadcastAbilityActivationChanged "/Game/Lyzandred/Blueprints/Characters/Abilities/DA_GroundPoundAbility.DA_GroundPoundAbility" false)
  (Animation|StopAnimMontage (Variables|Default|GetCharacterRef) (Variables|Default|GetGroundPoundMontage))
  (Variables|/Script/Project_Lyzandred.Lyz_TriformCharacter|SetbMovementInputEnabled _characterref true)
  (Variables|/Script/Project_Lyzandred.Lyz_TriformCharacter|SetbSwitchingCharactersEnabled _characterref true)
  (Variables|/Script/Engine.CharacterMovementComponent|SetGravityScale (Variables|Default|GetMovementComponentRef) (Variables|Default|GetDefaultGravity))
  (Variables|Default|SetbHasLanded true))

(event Custom|OnAttackHit
  (params (DamagedActor :type Actor%20Object%20Reference))
  (bind _returnvalue (Transformation|GetActorLocation DamagedActor))
  ;[0.15 0.15 0.15 0.5] Attack Hit
  ;;[0.15 0.15 0.15 0.5] Special Effects
  (Audio|PlaySoundatLocation "/Game/Lyzandred/Assets/SFX/SFX_SwordHit.SFX_SwordHit" _returnvalue "0, 0, 0" 1.0 1.0 0.0 0 0 0 0)
  (ForceFeedback|SpawnForceFeedbackatLocation "/Game/Lyzandred/Input/FF_SwordHit.FF_SwordHit" _returnvalue "0, 0, 0" false 1.0 0.0 0)
  (Class|Pawn|PawnMakeNoise (Variables|Default|GetCharacterRef) 5e+01 _returnvalue true 0)
  (CameraShakes|StartCameraShake (Variables|/Script/Engine.PlayerController|GetPlayerCameraManager (Game|GetPlayerController 0)) "/Game/Lyzandred/Blueprints/Effects/BP_SwordHitShake.BP_SwordHitShake_C" 1.0 "CameraLocal" "0, 0, 0"))

(event EventActivateAbility
  (bind _movementcomponentref (Variables|Default|GetMovementComponentRef))
  (bind _characterref (Variables|Default|GetCharacterRef))
  ;[0.15 0.15 0.15 0.5] Don't perform attack in wall slide
  (if (not (Class|LyzAbilityManagerComponent|IsAbilityStateActive (Variables|/Script/Project_Lyzandred.Lyz_TriformCharacter|GetAbilityManager (Variables|Default|GetCharacterRef)) "/Game/Lyzandred/Blueprints/Characters/Abilities/DA_WallSlideAbility.DA_WallSlideAbility"))
    (if (AI|Components|NavMovement|IsFalling (Variables|Default|GetMovementComponentRef))
      ;[0.15 0.15 0.15 0.5] Ground Pound Ability
      ;;[0.15 0.15 0.15 0.5] Set State
      (Class|LyzAbilityComponent|BroadcastAbilityActivationChanged "/Game/Lyzandred/Blueprints/Characters/Abilities/DA_GroundPoundAbility.DA_GroundPoundAbility" true)
      (Variables|Default|SetbIsGroundPounding true)
      (Variables|Default|SetbHasLanded false)
      ;;[0.15 0.15 0.15 0.5] Disable Movement and Character Switching
      (Variables|/Script/Project_Lyzandred.Lyz_TriformCharacter|SetbMovementInputEnabled _characterref false)
      (Variables|/Script/Project_Lyzandred.Lyz_TriformCharacter|SetbSwitchingCharactersEnabled _characterref false)
      ;;[0.15 0.15 0.15 0.5] Stop the character in the air before ground bound
      (Variables|/Script/Engine.CharacterMovementComponent|SetGravityScale _movementcomponentref 0.0)
      (Variables|/Script/Engine.MovementComponent|SetVelocity _movementcomponentref "0, 0, 0")
      (Audio|PlaySoundatLocation "/Game/Lyzandred/Assets/SFX/SFX_ShortSwing.SFX_ShortSwing" (Transformation|GetActorLocation (Components|GetOwner)) "0, 0, 0" 1.0 1.0 0.1 0 0 0 0)
      ;;[0.15 0.15 0.15 0.5] Play Animation montage and act on Notify when character enters correct pose
      (bind _notifyname (Animation|Montage|PlayMontage (Variables|/Script/Engine.Character|GetMesh (Variables|Default|GetCharacterRef)) (Variables|Default|GetGroundPoundMontage))
        (:OnNotifyBegin
          (if (== _notifyname "PoseReady")
            ;;[0.15 0.15 0.15 0.5] Restore Gravity and Launch Character downward
            (Variables|/Script/Engine.CharacterMovementComponent|SetGravityScale (Variables|Default|GetMovementComponentRef) (Variables|Default|GetDefaultGravity))
            (Character|LaunchCharacter (Variables|Default|GetCharacterRef) (Math|Vector|MakeVector 0.0 0.0 (Variables|Default|GetGroundPoundForce)) true true))))
      (else
        ;[0.15 0.15 0.15 0.5] Basic Swoird Attack Ability
        (if (not (Variables|Default|GetbIsAttackMontagePlaying))
          (Variables|Default|SetbIsAttackMontagePlaying true)
          (Variables|/Script/Project_Lyzandred.Lyz_TriformCharacter|SetbMovementInputEnabled (Variables|Default|GetCharacterRef) false)
          (bind _notifyname_2 (Animation|Montage|PlayMontage (Variables|/Script/Engine.Character|GetMesh (Variables|Default|GetCharacterRef)) (Variables|Default|GetAttackMontage))
            (:OnCompleted
              (Variables|Default|SetbIsAttackMontagePlaying false :!label _label)
              (Variables|/Script/Project_Lyzandred.Lyz_TriformCharacter|SetbMovementInputEnabled (Variables|Default|GetCharacterRef) true)
              (Default|AttackWindowClose (Variables|Default|GetMeleeAttackComponent) :!label _label_2))
            (:OnInterrupted
              (goto _label))
            (:OnNotifyBegin
              (switch name _notifyname_2
                (:AttackEnd
                  (goto _label_2))
                (:AttackStarted
                  (Default|AttackWindowOpen (Variables|Default|GetMeleeAttackComponent) (Variables|Default|GetWeaponComponent)))))))))))

(event EventTick
  (params (DeltaSeconds :type Float%20%28single-precision%29))
  ;[0.15 0.15 0.15 0.5] If we detect the character is going up, it means ground pound has ended
  (if (and (Variables|Default|GetbIsGroundPounding) (not (Variables|Default|GetbHasLanded)))
    (if (> (.z (Transformation|GetVelocity (Variables|Default|GetCharacterRef))) 0.0)
      (Variables|Default|SetbHasLanded true)
      (CallFunction|ExitGroundPound))))

(event EventOnAbilityEnabled
  (bind _characterref (Variables|Default|GetCharacterRef))
  (bind _returnvalue (Actor|GetComponentbyClass _characterref "/Game/Lyzandred/Blueprints/Characters/BP_MeleeAttackComponent.BP_MeleeAttackComponent_C"))
  ;[0.15 0.15 0.15 0.5] Initialization
  (|CallParentFunction)
  (EventDispatchers|BindEventtoLandedDelegate (Variables|Default|GetCharacterRef) (EventDispatchers|CreateEvent :!event Custom|OnCharacterLanded))
  (Variables|Default|SetDefaultGravity (Variables|/Script/Engine.CharacterMovementComponent|GetGravityScale (Variables|Default|GetMovementComponentRef)))
  (Variables|Default|SetWeaponComponent (Class|LyzTriformCharacter|GetAccessoryComponent (Variables|Default|GetCharacterRef) "RightHandAccessory"))
  (Utilities|IsValid _returnvalue
    (:Is%20Valid
      (bind _output_get (Variables|Default|SetMeleeAttackComponent _returnvalue))
      (EventDispatchers|BindEventtoOnAttackHit _output_get (EventDispatchers|CreateEvent :!event Custom|OnAttackHit)))))