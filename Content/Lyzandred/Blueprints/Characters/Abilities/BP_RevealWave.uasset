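; BP_RevealWave is a short-lived ability actor that plays an expanding sphere wave, spawned fresh for each use.
; Tick accumulates running time and uniformly scales the Reveal component linearly from zero toward TargetRadius over Duration, using ComputeCurrentScale.
; The actor destroys itself once Duration elapses, and does nothing on Tick if Duration is not positive.
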(event EventTick
  (params (DeltaSeconds :type Float%20%28single-precision%29))
  (bind _currentscale (CallFunction|ComputeCurrentScale))
  ;[0.15 0.15 0.15 0.5] Growing Sphere animation
  (if (> (Variables|Magic|GetDuration) 0.0)
    (Variables|Default|SetRunningTime (+ DeltaSeconds (Variables|Default|GetRunningTime)))
    (if (>= (Variables|Default|GetRunningTime) (Variables|Magic|GetDuration))
      ;[0.15 0.15 0.15 0.5] Destroy when done. Each time we will spawn a new Sphere
      (Actor|DestroyActor)
      (else
        (Transformation|SetRelativeScale3D (Variables|Default|GetReveal) (Math|Vector|MakeVector _currentscale _currentscale _currentscale))))))

(fn ConstructionScript)

(fn ComputeCurrentScale
  (return (* (/ (Variables|Default|GetRunningTime) (Variables|Magic|GetDuration)) (Variables|Magic|GetTargetRadius))))