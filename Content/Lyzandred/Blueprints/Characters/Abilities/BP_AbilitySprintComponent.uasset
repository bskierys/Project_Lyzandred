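; Sprint ability component that raises a character's walk speed while active.
; On enable it caches the movement component's default MaxWalkSpeed and binds to the character AbilityManager's activation-changed event.
; Activation multiplies the cached speed by SprintSpeedMultiplier, and deactivation restores it.
; A handler also deactivates sprint when the Slide ability ends.
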(event Custom|OnActivityDeactivated
  (params (Name :type Name) (Active :type Boolean))
  ;[0.15 0.15 0.15 0.5] Deactivate sprint at the end of the slide
  (if (and (== Name "Slide") (not Active))
    (Class|LyzAbilityComponent|DeactivateAbility)))

(event EventOnAbilityEnabled
  (bind _characterref (Variables|Default|GetCharacterRef))
  (|CallParentFunction)
  (Variables|Default|SetDefaultWalkSpeed (Variables|/Script/Engine.CharacterMovementComponent|GetMaxWalkSpeed (Variables|Default|GetMovementComponentRef)))
  (Utilities|IsValid _characterref
    (:Is%20Valid
      (EventDispatchers|BindEventtoOnAbilityActivationChanged (Variables|/Script/Project_Lyzandred.Lyz_TriformCharacter|GetAbilityManager _characterref) (EventDispatchers|CreateEvent :!event Custom|OnActivityDeactivated)))))

(event EventActivateAbility
  (|CallParentFunction)
  (Variables|/Script/Engine.CharacterMovementComponent|SetMaxWalkSpeed (Variables|Default|GetMovementComponentRef) (* (Variables|Default|GetDefaultWalkSpeed) (Variables|Default|GetSprintSpeedMultiplier))))

(event EventDeactivateAbility
  (|CallParentFunction)
  (Variables|/Script/Engine.CharacterMovementComponent|SetMaxWalkSpeed (Variables|Default|GetMovementComponentRef) (Variables|Default|GetDefaultWalkSpeed)))