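; Character ability component that performs a ground slide when sprinting at full speed, otherwise a flat dash.
; Slide temporarily scales walk speed, ending on timeout, montage interruption, deactivation or leaving the ground.
; Dash launches the character forward without gravity or movement input, scaling velocity and duration when sprinting, then brakes as its montage ends.
; Landing starts the cooldown that re-enables dashing; both moves broadcast ability activation changes.
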(event Custom|OnCharacterLanded
  (params (Hit :type Hit%20Result%20Structure%20%28by%20ref%29))
  ;[0.15 0.15 0.15 0.5] Restore ability to dash after the character has landed
  ;;[0.15 0.15 0.15 0.5] Apply cooldown to prevent dash spam on the ground
  (Utilities|Time|SetTimerbyEvent (EventDispatchers|CreateEvent :!event Custom|OnCooldownEnded) (Variables|Dash|GetDashCooldown))
  (Variables|Dash|SetbIsDashing false)
  (Class|LyzAbilityComponent|BroadcastAbilityActivationChanged (Variables|Default|GetAbilityData) false))

(event Custom|OnCooldownEnded
  ;[0.15 0.15 0.15 0.5] Reset flags
  (Variables|Dash|SetbHasDashed false))

(event Custom|OnMovementModeChange
  (params (Character :type Character%20Object%20Reference) (PrevMovementMode :type EMovementMode%20Enum :default "MOVE_None") (PreviousCustomMode :type Byte))
  (bind _movementcomponentref (Variables|Default|GetMovementComponentRef))
  ;[0.15 0.15 0.15 0.5] Cancel slide when start jump or falling
  (if (and (not (AI|Components|NavMovement|IsMovingonGround _movementcomponentref)) (Utilities|IsValid _movementcomponentref))
    (CallFunction|CancelSlide)))

(event Custom|CancelSlide
  ;[0.15 0.15 0.15 0.5] Activation
  ;;[0.15 0.15 0.15 0.5] Cancel Slide
  (if (Variables|GroundSlide|GetbIsSliding)
    (Variables|GroundSlide|SetbIsSliding false)
    (Variables|/Script/Engine.CharacterMovementComponent|SetMaxWalkSpeed (Variables|Default|GetMovementComponentRef) (Variables|Default|GetDefault%20Walk%20Speed))
    (Animation|StopAnimMontage (Variables|Default|GetCharacterRef) (Variables|GroundSlide|GetSlideMontage))
    (Class|LyzAbilityComponent|BroadcastAbilityActivationChanged "/Game/Lyzandred/Blueprints/Characters/Abilities/DA_SlideAbility.DA_SlideAbility" false)))

(event EventDeactivateAbility
  ;[0.15 0.15 0.15 0.5] Deactivation
  (if (Variables|GroundSlide|GetbIsSliding)
    (CallFunction|CancelSlide)))

(event EventActivateAbility
  (bind _movementcomponentref (Variables|Default|GetMovementComponentRef))
  ;[0.15 0.15 0.15 0.5] Activation
  (if (CallFunction|ShouldSlide)
    ;;[0.15 0.15 0.15 0.5] Sliding
    (Class|LyzAbilityComponent|BroadcastAbilityActivationChanged "/Game/Lyzandred/Blueprints/Characters/Abilities/DA_SlideAbility.DA_SlideAbility" true)
    (Variables|GroundSlide|SetbIsSliding true)
    (Variables|/Script/Engine.CharacterMovementComponent|SetMaxWalkSpeed (Variables|Default|GetMovementComponentRef) (* (Variables|Default|GetDefault%20Walk%20Speed) (Variables|GroundSlide|GetSlidingSpeedMultiplier)))
    (Animation|Montage|PlayMontage (Variables|/Script/Engine.Character|GetMesh (Variables|Default|GetCharacterRef)) (Variables|GroundSlide|GetSlideMontage)
      (:then
        (Utilities|FlowControl|Delay (Variables|GroundSlide|GetSlideDuration))
        (CallFunction|CancelSlide))
      (:OnInterrupted
        (CallFunction|CancelSlide)))
    (else
      ;;[0.15 0.15 0.15 0.5] Dashing
      ;;;[0.15 0.15 0.15 0.5] Guard against dash spam
      (if (not (Variables|Dash|GetbHasDashed))
        (Variables|Dash|SetbHasDashed true)
        (Class|LyzAbilityComponent|BroadcastAbilityActivationChanged (Variables|Default|GetAbilityData) true)
        ;;;[0.15 0.15 0.15 0.5] Raise the dashing flag
        (Variables|Dash|SetbIsDashing true)
        (Variables|/Script/Project_Lyzandred.Lyz_TriformCharacter|SetbMovementInputEnabled (Variables|Default|GetCharacterRef) false)
        ;;;[0.15 0.15 0.15 0.5] Reset the velocity and temporarily disable gravity, to ensure we dash in a flat plane.
        (Variables|/Script/Engine.CharacterMovementComponent|SetGravityScale (Variables|/Script/Engine.Character|GetCharacterMovement (Variables|Default|GetCharacterRef)) 0.0)
        (Character|LaunchCharacter (Variables|Default|GetCharacterRef) (CallFunction|ComputeDashVelocity) true true)
        (Animation|Montage|PlayMontage (Variables|/Script/Engine.Character|GetMesh (Variables|Default|GetCharacterRef)) (Variables|Dash|GetDashMontage)
          (:then
            ;;;[0.15 0.15 0.15 0.5] Stop Dashing after time - depends on the movement flags
            (Utilities|FlowControl|Delay (CallFunction|ComputeDashDuration))
            (Animation|StopAnimMontage (Variables|Default|GetCharacterRef) (Variables|Dash|GetDashMontage)))
          (:OnCompleted
            ;;;[0.15 0.15 0.15 0.5] When Dash ends slow down character movement
            (Variables|/Script/Engine.MovementComponent|SetVelocity _movementcomponentref (/ (Variables|/Script/Engine.MovementComponent|GetVelocity _movementcomponentref) (Variables|Dash|GetDashOpposingForce)) :!label _label)
            ;;;[0.15 0.15 0.15 0.5] When the dash animation completes, restore gravity.
            (Variables|/Script/Engine.CharacterMovementComponent|SetGravityScale _movementcomponentref (Variables|Default|GetDefaultGravity))
            ;;;[0.15 0.15 0.15 0.5] Lower the dashing flag
            (Variables|Dash|SetbIsDashing false)
            (Variables|/Script/Project_Lyzandred.Lyz_TriformCharacter|SetbMovementInputEnabled (Variables|Default|GetCharacterRef) true))
          (:OnInterrupted
            (goto _label)))))))

(event EventOnAbilityDisabled
  ;[0.15 0.15 0.15 0.5] Notify about deactivation
  (Class|LyzAbilityComponent|BroadcastAbilityActivationChanged (Variables|Default|GetAbilityData) false))

(event EventOnAbilityEnabled
  (bind _movementcomponentref (Variables|Default|GetMovementComponentRef))
  (bind _characterref (Variables|Default|GetCharacterRef))
  ;[0.15 0.15 0.15 0.5] Initialization
  (|CallParentFunction)
  ;;[0.15 0.15 0.15 0.5] Subscribe to On Landed Event
  (Utilities|IsValid _characterref
    (:Is%20Valid
      (EventDispatchers|BindEventtoLandedDelegate _characterref (EventDispatchers|CreateEvent :!event Custom|OnCharacterLanded))
      ;[0.15 0.15 0.15 0.5] Subscribe to movement mode change to prevent slide-jumping and falling
      (Character|BindEventtoMovementModeChangedDelegate (Variables|Default|GetCharacterRef) (EventDispatchers|CreateEvent :!event Custom|OnMovementModeChange))
      ;[0.15 0.15 0.15 0.5] Set default values to reset them later
      (Utilities|IsValid _movementcomponentref
        (:Is%20Valid
          (Variables|Default|SetDefault%20Walk%20Speed (Variables|/Script/Engine.CharacterMovementComponent|GetMaxWalkSpeed _movementcomponentref))
          (Variables|Default|SetDefaultGravity (Variables|/Script/Engine.CharacterMovementComponent|GetGravityScale (Variables|Default|GetMovementComponentRef))))))))

(fn ComputeDashVelocity
  (return (* (* (Transformation|GetActorForwardVector (Variables|Default|GetCharacterRef)) "1.000000,1.000000,0.000000") (Variables|Dash|GetDashVelocityBase) (Math|Float|SelectFloat (Variables|Dash|GetDashSprintMultiplier) 1.0 (CallFunction|IsinSprint)))))

(fn ComputeDashDuration
  (return (* (Variables|Dash|GetDashDuration) (Math|Float|SelectFloat (Variables|Dash|GetDashSprintMultiplier) 1.0 (CallFunction|IsinSprint)))))

(fn CanbeActivated
  (params (ActiveAbilities :type Set%20of%20Names))
  (return true))

(fn ShouldSlide
  (bind _movementcomponentref (Variables|Default|GetMovementComponentRef))
  (return (Math|Boolean|ANDBoolean (CallFunction|IsinSprint) (AI|Components|NavMovement|IsMovingonGround _movementcomponentref) (Math|Float|NearlyEqual(Float) (Math|Vector|VectorLength (Variables|/Script/Engine.MovementComponent|GetVelocity _movementcomponentref)) (Variables|/Script/Engine.CharacterMovementComponent|GetMaxWalkSpeed _movementcomponentref) 0.1))))

(fn IsinSprint
  (return (Class|LyzAbilityManagerComponent|IsAbilityStateActive (Variables|/Script/Project_Lyzandred.Lyz_TriformCharacter|GetAbilityManager (Variables|Default|GetCharacterRef)) "/Game/Lyzandred/Blueprints/Characters/Abilities/DA_SprintAbility.DA_SprintAbility")))