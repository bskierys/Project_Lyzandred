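; BP_ReportTouchComponent is a component for Character actors that turns physical contact into AI touch sense events.
; On BeginPlay it binds to the owning character's capsule overlap.
; Each overlap reports a touch event with the overlapped actor as receiver, passing the owner and its location.
; A separate CreateLockedText function merges "why locked" messages from supplied components into one text, unconnected to the touch logic.
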(event Custom|OnBeginOverlap
  (params (OverlappedComponent :type Primitive%20Component%20Object%20Reference) (OtherActor :type Actor%20Object%20Reference) (OtherComp :type Primitive%20Component%20Object%20Reference) (OtherBodyIndex :type Integer) (bFromSweep :type Boolean) (SweepResult :type Hit%20Result%20Structure%20%28by%20ref%29))
  (bind _character_ref (Variables|Default|GetCharacter%20Ref))
  (Class|AISenseTouch|ReportTouchEvent OtherActor _character_ref (Transformation|GetActorLocation _character_ref)))

(event EventBeginPlay
  ;[0.15 0.15 0.15 0.5] Initialization
  (bind _output_get (Variables|Default|SetCharacter%20Ref (.AsCharacter (Utilities|Casting|CastToCharacter (Components|GetOwner)))))
  (Collision|BindEventtoOnComponentBeginOverlap (Variables|/Script/Engine.Character|GetCapsuleComponent _output_get) (EventDispatchers|CreateEvent :!event Custom|OnBeginOverlap)))

(fn CreateLockedText
  (params (Components :type Array%20of%20BP%20Unlockable%20Component%20Object%20References))
  (for _array_element Components
    (bind _message (Default|CreateWhyLockedMessage _array_element))
    (Utilities|Array|Add (LocalVariables|GetTextArray) _message))
  (bind _message_2 (CallFunction|ArrayOfTextstoText (LocalVariables|GetTextArray)))
  (return _message_2))