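; Main menu game mode that shows the menu widget and handles starting or quitting the game.
; On BeginPlay it creates WBP_MainMenu, gives it a reference to itself, and switches to game-and-UI input with a visible cursor.
; Its StartGame event restores game-only input, hides the cursor and opens L_MainLevel, while QuitGame exits the application.
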(event Custom|StartGame
  (bind _returnvalue (Game|GetPlayerController 0))
  (Input|SetInputModeGameOnly _returnvalue false)
  (Variables|/Script/Engine.PlayerController|SetbShowMouseCursor _returnvalue false)
  (Game|OpenLevel(byObjectReference) "/Game/Lyzandred/Maps/L_MainLevel.L_MainLevel"))

(event Custom|QuitGame
  (Game|QuitGame (Game|GetPlayerController 0) "Quit" false))

(event EventBeginPlay
  (bind _returnvalue (Game|GetPlayerController 0))
  (bind _returnvalue_2 (UserInterface|CreateWidget "/Game/Lyzandred/Blueprints/Widgets/WBP_MainMenu.WBP_MainMenu_C" (Game|GetPlayerController 0)))
  (bind _output_get (Variables|Default|SetMainMenuWidget _returnvalue_2))
  (Variables|/Game/Lyzandred/Blueprints/Widgets/WBP_MainMenu.WBP_MainMenu_C|SetMainMenuGameMode _output_get self)
  (UserInterface|Viewport|AddtoViewport _output_get 0)
  (Input|SetInputModeGameandUI _returnvalue (Variables|Default|GetMainMenuWidget) "DoNotLock" false false)
  (Variables|/Script/Engine.PlayerController|SetbShowMouseCursor _returnvalue true))

(fn ConstructionScript)