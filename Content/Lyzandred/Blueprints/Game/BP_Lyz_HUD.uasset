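; HUD Blueprint for Lyzandred that creates and owns the on-screen level HUD and timer widgets.
; On BeginPlay it adds both widgets to the first player's viewport and keeps references, with the timer starting hidden.
; Custom events set visibility for the timer alone or for both widgets together, so showing the whole HUD also reveals the timer.
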(event EventBeginPlay
  ;[0.15 0.15 0.15 0.5] Main Hud Widget
  (bind _returnvalue (UserInterface|CreateWidget "/Game/Lyzandred/Blueprints/Widgets/WBP_LevelHud.WBP_LevelHud_C" (Game|GetPlayerController 0)))
  (bind _output_get (Variables|Default|SetLevelHud _returnvalue))
  (UserInterface|Viewport|AddtoViewport _output_get 0)
  ;[0.15 0.15 0.15 0.5] On Screen Timer
  (bind _returnvalue_2 (UserInterface|CreateWidget "/TimerPlugin/WBP_TimerDefault.WBP_TimerDefault_C" (Game|GetPlayerController 0)))
  (bind _output_get_2 (Variables|Default|SetTimerWidget _returnvalue_2))
  (UserInterface|Viewport|AddtoViewport _output_get_2 0)
  (Widget|SetVisibility (Variables|Default|GetTimerWidget) "Hidden"))

(event EventSetTimerVisibility
  (params (Visibility :type ESlateVisibility%20Enum :default "Visible"))
  (Widget|SetVisibility (Variables|Default|GetTimerWidget) Visibility))

(event EventSetHudVisibility
  (params (Visibility :type ESlateVisibility%20Enum :default "Visible"))
  ;[0.15 0.15 0.15 0.5] Show/Hide HUD
  (Widget|SetVisibility (Variables|Default|GetLevelHud) Visibility)
  (Widget|SetVisibility (Variables|Default|GetTimerWidget) Visibility))

(fn ConstructionScript)