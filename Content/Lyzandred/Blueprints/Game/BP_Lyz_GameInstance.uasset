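; BP_Lyz_GameInstance is the Lyzandred game instance, providing a wallet that records the coins collected in the game.
; AddCoin takes a coin class, reads its Value from the class defaults and adds it to the running total.
; It also increments that class's count in the CollectedCoins map, creating the entry if absent, then returns the updated total.
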(fn AddCoin
  (params (CoinType :type Lyz%20Coin%20Type%20Class%20Reference))
  ;[0.15 0.15 0.15 0.5] Update current wallate with new coin value
  (Variables|Default|SetCollectedCoinsValue (+ (Variables|Default|GetCollectedCoinsValue) (.Value (Utilities|GetClassDefaults CoinType))))
  (Utilities|FlowControl|Sequence
    (:then_0
      ;[0.15 0.15 0.15 0.5] Update the info on types and number of coins in our wallet
      (if (Utilities|Map|Contains (Variables|Default|GetCollectedCoins) CoinType)
        (bind _result (Math|Integer|IncrementInt (.Value (Utilities|Map|Find (Variables|Default|GetCollectedCoins) CoinType)))
          (:%20%20
            (Utilities|Map|Add (Variables|Default|GetCollectedCoins) CoinType _result)))
        (else
          (Utilities|Map|Add (Variables|Default|GetCollectedCoins) CoinType 1))))
    (:then_1
      (return (Variables|Default|GetCollectedCoinsValue)))))