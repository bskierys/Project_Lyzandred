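; Bouncy mushroom platforming actor that launches any Character overlapping it upward and plays a bounce sound.
; Launch Z velocity scales with the character's incoming speed plus a base bounce, clamped between minimum and maximum, and overrides existing Z.
; A squash-stretch timeline drives the mesh's X and Y scale.
; Z scale stays at one for positive timeline values, as the reciprocal is selected only otherwise.
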(event Collision|EventActorBeginOverlap
  (params (OtherActor :type Actor%20Object%20Reference))
  ;[0.15 0.15 0.15 0.5] Bounce Character
  (bind _ascharacter (Utilities|Casting|CastToCharacter OtherActor))
  (Character|LaunchCharacter _ascharacter (Math|Vector|MakeVector 0.0 0.0 (Math|Float|Clamp(Float) (+ (* (Math|Float|Absolute(Float) (Math|Vector|VectorLength (Transformation|GetVelocity _ascharacter))) (Variables|Default|GetBouceMultiplier)) (Variables|Default|GetBaseBounce)) (Variables|Default|GetMinBounce) (Variables|Default|GetMaxBounce))) false true)
  ;[0.15 0.15 0.15 0.5] Sound Effect
  (Audio|PlaySoundatLocation "/Game/Lyzandred/Assets/SFX/SFX_bounce_Cue.SFX_bounce_Cue" (Transformation|GetActorLocation) "0, 0, 0" 1.0 1.0 0.0 0 0 0 0)
  ;[0.15 0.15 0.15 0.5] Stretch Animation
  (bind _scalevalue (Timeline|TL_SquashStretch PlayFromStart)
    (:Update
      (Transformation|SetRelativeScale3D (Variables|Default|GetBouncyMesh) (Math|Vector|MakeVector _scalevalue _scalevalue (Math|Float|SelectFloat 1.0 (/ 1.0 _scalevalue) (> _scalevalue 0.0)))))))

(fn ConstructionScript)